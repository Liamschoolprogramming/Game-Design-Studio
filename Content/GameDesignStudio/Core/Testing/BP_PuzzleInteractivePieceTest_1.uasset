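; A test Blueprint, named as a puzzle interactive piece, holding scratch calls to GameManagerSubsystem.
; BeginPlay and the construction script are empty, and every other node chain is disconnected, so none of it runs.
; The unused chains look up PuzzleRiverManager, print its CalculateValues result and call SnapshotActorValues, once after a delay.
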(event EventBeginPlay)

(fn ConstructionScript)