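; Player controller Blueprint that links menu and possession input to BP_HUD in a game where the player possesses entities such as Golems, Beetles and Turrets.
; Enhanced Input actions toggle menus, cycle possession slots and confirm possession, while input device changes trigger a control-device check.
; Hotbar functions keep the HUD in sync with nearby possessable entities, resolving the newest entry's icon from a data table by character type.
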(event Custom|OnInputHardwareDeviceChanged_Event
  (params (UserId :type Platform%20User%20Id%20Structure) (DeviceId :type Input%20Device%20Id%20Structure))
  (Class|PlayerControllerBase|CheckControlDevice UserId DeviceId))

(event Input|EnhancedActionEvents|EnhancedInputActionIA_Inventory
  (params (ActionValue :type Boolean) (ElapsedSeconds :type Float%20%28double-precision%29) (TriggeredSeconds :type Float%20%28double-precision%29) (InputAction :type Input%20Action%20Object%20Reference :default "/Game/GameDesignStudio/Input/Actions/IA_Inventory.IA_Inventory"))
  (:Completed
    (Default|ToggleInventory (Variables|Default|GetHUD))))

(event Input|EnhancedActionEvents|EnhancedInputActionIA_PlayerStats
  (params (ActionValue :type Boolean) (ElapsedSeconds :type Float%20%28double-precision%29) (TriggeredSeconds :type Float%20%28double-precision%29) (InputAction :type Input%20Action%20Object%20Reference :default "/Game/GameDesignStudio/Input/Actions/IA_PlayerStats.IA_PlayerStats"))
  (:Completed
    (Default|TogglePlayerStats (Variables|Default|GetHUD))))

(event Input|EnhancedActionEvents|EnhancedInputActionIA_PauseGame
  (params (ActionValue :type Boolean) (ElapsedSeconds :type Float%20%28double-precision%29) (TriggeredSeconds :type Float%20%28double-precision%29) (InputAction :type Input%20Action%20Object%20Reference :default "/Game/GameDesignStudio/Input/Actions/IA_PauseGame.IA_PauseGame"))
  (Default|TogglePauseMenu (Variables|Default|GetHUD)))

(event Input|EnhancedActionEvents|EnhancedInputActionIA_QuestMenu
  (params (ActionValue :type Boolean) (ElapsedSeconds :type Float%20%28double-precision%29) (TriggeredSeconds :type Float%20%28double-precision%29) (InputAction :type Input%20Action%20Object%20Reference :default "/Game/GameDesignStudio/Input/Actions/IA_QuestMenu.IA_QuestMenu"))
  (:Completed
    (Default|ToggleQuestMenu (Variables|Default|GetHUD))))

(event Input|EnhancedActionEvents|EnhancedInputActionIA_CycleUp
  (params (ActionValue :type Boolean) (ElapsedSeconds :type Float%20%28double-precision%29) (TriggeredSeconds :type Float%20%28double-precision%29) (InputAction :type Input%20Action%20Object%20Reference :default "/Game/GameDesignStudio/Input/Actions/IA_CycleUp.IA_CycleUp"))
  (Default|OnCyclePossessableSlot (Variables|Default|GetHUD) (Variables|Default|GetIndexForPossessables)))

(event Input|EnhancedActionEvents|EnhancedInputActionIA_ConfirmPossession
  (params (ActionValue :type Boolean) (ElapsedSeconds :type Float%20%28double-precision%29) (TriggeredSeconds :type Float%20%28double-precision%29) (InputAction :type Input%20Action%20Object%20Reference :default "/Game/GameDesignStudio/Input/Actions/IA_ConfirmPossession.IA_ConfirmPossession"))
  (Class|PlayerControllerBase|ConfirmPossession)
  (Default|OnConfirmPossession (Variables|Default|GetHUD)))

(event EventBeginPlay
  (EventDispatchers|AssignOnInputHardwareDeviceChanged (|InputDeviceSubsystem) (delegate Custom|OnInputHardwareDeviceChanged_Event))
  (bind _asbp_hud (Utilities|Casting|CastToBP_HUD (HUD|GetHUD)))
  (Variables|Default|SetHUD _asbp_hud))

(fn ConstructionScript)

(fn RemovePossessablefromHotbar
  (params (IndexToRemove :type Integer))
  (Default|RemovePossessablefromHotbar (Variables|Default|GetHUD) IndexToRemove))

(fn AddPossessabletoHotbar
  (LocalVariables|SetL_PossssableIndex (- (Utilities|Array|Length (Variables|Default|GetClosestPossessableEntities)) 1))
  (switch Utilities|FlowControl|Switch|SwitchonEPlayerCharacterType (Variables|/Script/GameDesignStudio.PlayerCharacter|GetPlayerCharacterType (Utilities|Array|Get(acopy) (Variables|Default|GetClosestPossessableEntities) (LocalVariables|GetL_PossssableIndex)))
    (:Default
      (LocalVariables|SetL_PossessableType "Default"))
    (:Golem
      (LocalVariables|SetL_PossessableType "Golem"))
    (:Beetle
      (LocalVariables|SetL_PossessableType "Beetle"))
    (:Turret
      (LocalVariables|SetL_PossessableType "Turret")))
  (bind _returnvalue (Utilities|GetDataTableRow "/Game/GameDesignStudio/Possessables/DT_PlayerCharacterTypeIcon.DT_PlayerCharacterTypeIcon" (LocalVariables|GetL_PossessableType))
    (:then
      (Default|AddPossessabletoHotbar (Variables|Default|GetHUD) (.icon _returnvalue) (LocalVariables|GetL_PossssableIndex)))))

(fn OnCyclePossessionTarget
  (Default|OnCyclePossessableSlot (Variables|Default|GetHUD) (Variables|Default|GetIndexForPossessables)))

(fn CanPossessPossessableEntity
  (params (Entity%20to%20Check :type Possessable%20Entity%20Object%20Reference))
  (bind _can_possess (CallFunction|CanPossessPossessableEntity Entity%20to%20Check))
  (return _can_possess))

(fn GetPossessionTimerHandle
  (return (Variables|Default|GetPossessionTimerHandle)))