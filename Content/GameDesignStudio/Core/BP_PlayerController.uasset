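; Player controller for the possession mechanic, routing Enhanced Input to menus and to cycling, number-key selection and confirmation of possession targets.
; It mirrors possessable entities into HUD hotbar slots with data-table icons, highlights the selected one and throttles out-of-sight warnings by timer.
; It also spawns stat-boost rewards and level portals at the first reward zone, rechecks input device on hardware changes, and has level-jump debug keys.
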(event Custom|OnInputHardwareDeviceChanged_Event
  (params (UserId :type Platform%20User%20Id%20Structure) (DeviceId :type Input%20Device%20Id%20Structure))
  (Class|PlayerControllerBase|CheckControlDevice UserId DeviceId))

(event Custom|ResetOutOfSightWarningTimer
  (Variables|Default|SetShowOutOfSightWarning true))

(event Input|EnhancedActionEvents|EnhancedInputActionIA_Inventory
  (params (ActionValue :type Boolean) (ElapsedSeconds :type Float%20%28double-precision%29) (TriggeredSeconds :type Float%20%28double-precision%29) (InputAction :type Input%20Action%20Object%20Reference :default "/Game/GameDesignStudio/Input/Actions/IA_Inventory.IA_Inventory"))
  (:Completed
    (Default|ToggleInventory (Variables|Default|GetHUD))))

(event Input|EnhancedActionEvents|EnhancedInputActionIA_PlayerStats
  (params (ActionValue :type Boolean) (ElapsedSeconds :type Float%20%28double-precision%29) (TriggeredSeconds :type Float%20%28double-precision%29) (InputAction :type Input%20Action%20Object%20Reference :default "/Game/GameDesignStudio/Input/Actions/IA_PlayerStats.IA_PlayerStats"))
  (:Completed
    (Default|TogglePlayerStats (Variables|Default|GetHUD))))

(event Input|EnhancedActionEvents|EnhancedInputActionIA_PauseGame
  (params (ActionValue :type Boolean) (ElapsedSeconds :type Float%20%28double-precision%29) (TriggeredSeconds :type Float%20%28double-precision%29) (InputAction :type Input%20Action%20Object%20Reference :default "/Game/GameDesignStudio/Input/Actions/IA_PauseGame.IA_PauseGame"))
  (:Completed
    (Default|TogglePauseMenu (Variables|Default|GetHUD) false false)))

(event Input|EnhancedActionEvents|EnhancedInputActionIA_QuestMenu
  (params (ActionValue :type Boolean) (ElapsedSeconds :type Float%20%28double-precision%29) (TriggeredSeconds :type Float%20%28double-precision%29) (InputAction :type Input%20Action%20Object%20Reference :default "/Game/GameDesignStudio/Input/Actions/IA_QuestMenu.IA_QuestMenu"))
  (:Completed
    (Default|ToggleQuestMenu (Variables|Default|GetHUD))))

(event Input|EnhancedActionEvents|EnhancedInputActionIA_CycleUp
  (params (ActionValue :type Boolean) (ElapsedSeconds :type Float%20%28double-precision%29) (TriggeredSeconds :type Float%20%28double-precision%29) (InputAction :type Input%20Action%20Object%20Reference :default "/Game/GameDesignStudio/Input/Actions/IA_CycleUp.IA_CycleUp"))
  (CallFunction|OnCyclePossessionTarget))

(event Input|EnhancedActionEvents|EnhancedInputActionIA_ConfirmPossession
  (params (ActionValue :type Boolean) (ElapsedSeconds :type Float%20%28double-precision%29) (TriggeredSeconds :type Float%20%28double-precision%29) (InputAction :type Input%20Action%20Object%20Reference :default "/Game/GameDesignStudio/Input/Actions/IA_ConfirmPossession.IA_ConfirmPossession"))
  (Class|PlayerControllerBase|ConfirmPossession))

(event Input|EnhancedActionEvents|EnhancedInputActionIA_SetPossessIndexByNumber
  (params (ActionValue :type Vector%202D%20Structure) (ElapsedSeconds :type Float%20%28double-precision%29) (TriggeredSeconds :type Float%20%28double-precision%29) (InputAction :type Input%20Action%20Object%20Reference :default "/Game/GameDesignStudio/Input/Actions/IA_SetPossessIndexByNumber.IA_SetPossessIndexByNumber"))
  (for _array_element (Class|EnhancedInputSubsystemInterface|QueryKeysMappedtoAction (PlayerController|LocalPlayerSubsystems|GetEnhancedInputLocalPlayerSubsystem) InputAction)
    (if (Game|Player|IsInputKeyDown _array_element)
      (Class|PlayerControllerBase|SetPossessIndexbyNumber (Utilities|String|ToString(Text) (Class|KismetInputLibrary|KeyGetDisplayName _array_element true))))))

(event EventBeginPlay
  (EventDispatchers|AssignOnInputHardwareDeviceChanged (|InputDeviceSubsystem) (delegate Custom|OnInputHardwareDeviceChanged_Event))
  (bind _asbp_hud (Utilities|Casting|CastToBP_HUD (HUD|GetHUD)))
  (Variables|Default|SetHUD _asbp_hud))

(event EventOnTrytoPossessOutOfSight
  (if (Variables|Default|GetShowOutOfSightWarning)
    (Default|DisplayPopupNotification (Variables|Default|GetHUD) (Utilities|Struct|MakeDataTableRowHandle "/Game/GameDesignStudio/Tutorial/DT_Hints.DT_Hints" "OutOfSight"))
    (Variables|Default|SetShowOutOfSightWarning false)
    (Utilities|Time|SetTimerbyEvent (delegate Custom|ResetOutOfSightWarningTimer) 5.0)))

(event Input|KeyboardEvents|CtrlH
  (params (Key :type Key%20Structure))
  (:Pressed
    (Game|OpenLevel(byObjectReference) "/Game/GameDesignStudio/Maps/Hub.Hub")))

(event Input|KeyboardEvents|CtrlT
  (params (Key :type Key%20Structure))
  (:Pressed
    (Game|OpenLevel(byObjectReference) "/Game/GameDesignStudio/Maps/Tutorial.Tutorial")))

(fn ConstructionScript
  (Variables|Default|SetPossessionWidget "/Game/GameDesignStudio/UI/PossessTimerBar/WBP_PossessTimerBar.WBP_PossessTimerBar_C"))

(fn RemovePossessablefromHotbar
  (params (IndexToRemove :type Integer))
  (Default|RemovePossessablefromHotbar (Variables|Default|GetHUD) IndexToRemove))

(fn AddPossessabletoHotbar
  (LocalVariables|SetL_PossessableIndex (- (Utilities|Array|Length (Variables|Default|GetClosestPossessableEntities)) 1))
  (switch Utilities|FlowControl|Switch|SwitchonEPlayerCharacterType (Variables|/Script/GameDesignStudio.PlayerCharacter|GetPlayerCharacterType (Utilities|Array|Get(acopy) (Variables|Default|GetClosestPossessableEntities) (LocalVariables|GetL_PossessableIndex)))
    (:Default
      (LocalVariables|SetL_PossessableType "Default"))
    (:Golem
      (LocalVariables|SetL_PossessableType "Golem"))
    (:Beetle
      (LocalVariables|SetL_PossessableType "Beetle"))
    (:Turret
      (LocalVariables|SetL_PossessableType "Turret")))
  (bind _returnvalue (Utilities|GetDataTableRow "/Game/GameDesignStudio/Possessables/DT_PlayerCharacterTypeIcon.DT_PlayerCharacterTypeIcon" (LocalVariables|GetL_PossessableType))
    (:then
      (Default|AddPossessabletoHotbar (Variables|Default|GetHUD) (.icon _returnvalue) (LocalVariables|GetL_PossessableIndex)))))

(fn OnCyclePossessionTarget
  (Default|OnCyclePossessableSlot (Variables|Default|GetHUD) (Variables|Default|GetIndexForPossessables))
  (for (_array_element _array_index) (Variables|Default|GetClosestPossessableEntities)
    (Class|PossessableEntity|OnSetHighlight _array_element (== _array_index (Variables|Default|GetIndexForPossessables)))))

(fn OnReturntoPlayer
  (Default|ResetHighlights (Variables|Default|GetHUD)))

(fn SpawnPortal
  (params (LevelTarget :type World%20Soft%20Object%20Reference))
  (bind _returnvalue (Class|PlayerControllerBase|FindFirstRewardSpawnZone))
  (Utilities|IsValid _returnvalue
    (:Is%20Valid
      (bind _returnvalue_2 (Game|SpawnActorfromClass "/Game/GameDesignStudio/Warps/BP_PortalWarp.BP_PortalWarp_C" (Transformation|GetActorTransform _returnvalue) "Undefined" "MultiplyWithRoot" 0 0))
      (Variables|/Game/GameDesignStudio/Warps/BP_PortalWarp.BP_PortalWarp_C|SetLevel _returnvalue_2 LevelTarget))))

(fn GriefRemoveTutorial
  (Class|PuzzleGriefManager|DisableAllGriefObjects (Class|GameManagerSubsystem|GetPuzzleTutorialGriefManager (Subsystems|GetGameManagerSubsystem)))
  (Development|PrintString "Called Grief" true true "(R=1.000000,G=0.308281,B=0.282491,A=1.000000)" 1e+01))

(fn GiveReward
  (params (BoostAmount :type Float%20%28single-precision%29) (StatToBoost :type String))
  (bind _returnvalue (Class|PlayerControllerBase|FindFirstRewardSpawnZone))
  (Utilities|IsValid _returnvalue
    (:Is%20Valid
      (switch string StatToBoost
        (:Health
          (Game|SpawnActorfromClass "/Game/GameDesignStudio/Puzzle/Reward/BP_RewardPickupable.BP_RewardPickupable_C" (Transformation|GetActorTransform _returnvalue) "Undefined" "MultiplyWithRoot" 0 "Health" BoostAmount 0))
        (:Stamina
          (Game|SpawnActorfromClass "/Game/GameDesignStudio/Puzzle/Reward/BP_RewardPickupable.BP_RewardPickupable_C" (Transformation|GetActorTransform _returnvalue) "Undefined" "MultiplyWithRoot" 0 "Stamina" BoostAmount 0))
        (:Mind
          (Game|SpawnActorfromClass "/Game/GameDesignStudio/Puzzle/Reward/BP_RewardPickupable.BP_RewardPickupable_C" (Transformation|GetActorTransform _returnvalue) "Undefined" "MultiplyWithRoot" 0 "Mind" BoostAmount 0))))))

(fn CanPossessPossessableEntity
  (params (Entity%20to%20Check :type Possessable%20Entity%20Object%20Reference))
  (bind _can_possess (CallFunction|CanPossessPossessableEntity Entity%20to%20Check))
  (return _can_possess))

(fn GetBPPlayerController
  (return self))

(fn GetPossessionTimerHandle
  (return (Variables|Default|GetPossessionTimerHandle)))