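; Game instance Blueprint that relays music and settings calls and restores saved state after loading.
; Interface events forward to music playback and audio or other settings save and load functions.
; On LoadDone it waits a frame, loads puzzles and settings, applies the control scheme, then loads save stations.
; SwitchControlScheme swaps Enhanced Input mapping contexts on the player controller between left-handed and right-handed layouts, removing the default context.
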(event EventInit
  (|CallParentFunction))

(event EventIPlayMusic
  (params (Music :type Sound%20Base%20Object%20Reference) (FadeOutTimeOld :type Float%20%28double-precision%29) (FadeInTimeNew :type Float%20%28double-precision%29))
  (Class|ELSGameInstance|PlayMusic Music FadeOutTimeOld FadeInTimeNew))

(event EventIStopMusic
  (params (FadeOutTime :type Float%20%28double-precision%29))
  (Class|ELSGameInstance|StopMusic FadeOutTime))

(event EventIPauseMusic
  (Class|ELSGameInstance|PauseMusic))

(event EventIResumeMusic
  (Class|ELSGameInstance|ResumeMusic))

(event EventILoadAudioSettings
  (Class|ELSGameInstance|LoadAudioSettings))

(event EventISaveAudioSettings
  (params (Music%20Volume :type Float%20%28double-precision%29) (SFX%20Volume :type Float%20%28double-precision%29) (Master%20Volume :type Float%20%28double-precision%29))
  (Class|ELSGameInstance|SaveAudioSettings Music%20Volume SFX%20Volume Master%20Volume))

(event EventLoadDone
  (Utilities|FlowControl|DelayUntilNextFrame)
  (Class|SaveSubsystem|LoadPuzzles (Subsystems|GetSaveSubsystem))
  (bind _returnvalue (Class|ELSGameInstance|LoadOtherSettings))
  (CallFunction|SwitchControlScheme (Variables|/Script/GameDesignStudio.SettingsSaveGame|GetbUseLeftHandedControls _returnvalue))
  (Class|SaveStationManager|LoadSaveStations (Class|GameManagerSubsystem|GetSaveStationManager (Subsystems|GetGameManagerSubsystem))))

(event EventISaveOtherSettings
  (Class|ELSGameInstance|SaveOtherSettings (Variables|Default|GetLeftHandedControls)))

(event EventISwitchControlScheme
  (params (UseLeftHanded :type Boolean))
  (bind _output_get (Variables|Default|SetLeftHandedControls UseLeftHanded))
  (CallFunction|SwitchControlScheme _output_get))

(fn SwitchControlScheme
  (params (Condition :type Boolean))
  (if Condition
    (bind _asbp_player_controller (Utilities|Casting|CastToBP_PlayerController (Game|GetPlayerController 0)))
    (Utilities|FlowControl|Sequence
      (:then_0
        (Input|RemoveMappingContext (PlayerController|LocalPlayerSubsystems|GetEnhancedInputLocalPlayerSubsystem _asbp_player_controller) (Variables|Default|GetDefaultMappingContext) "(bIgnoreAllPressedKeysUntilRelease=True,bForceImmediately=False,bNotifyUserSettings=False)"))
      (:then_1
        (Input|RemoveMappingContext (PlayerController|LocalPlayerSubsystems|GetEnhancedInputLocalPlayerSubsystem _asbp_player_controller) (Variables|Default|GetRightHandedMappingContext) "(bIgnoreAllPressedKeysUntilRelease=True,bForceImmediately=False,bNotifyUserSettings=False)"))
      (:then_2
        (Input|AddMappingContext (PlayerController|LocalPlayerSubsystems|GetEnhancedInputLocalPlayerSubsystem _asbp_player_controller) (Variables|Default|GetLeftHandedMappingContext) 0 "(bIgnoreAllPressedKeysUntilRelease=True,bForceImmediately=False,bNotifyUserSettings=False)")))
    (else
      (bind _asbp_player_controller_2 (Utilities|Casting|CastToBP_PlayerController (Game|GetPlayerController 0)))
      (Utilities|FlowControl|Sequence
        (:then_0
          (Input|RemoveMappingContext (PlayerController|LocalPlayerSubsystems|GetEnhancedInputLocalPlayerSubsystem _asbp_player_controller_2) (Variables|Default|GetDefaultMappingContext) "(bIgnoreAllPressedKeysUntilRelease=True,bForceImmediately=False,bNotifyUserSettings=False)"))
        (:then_1
          (Input|RemoveMappingContext (PlayerController|LocalPlayerSubsystems|GetEnhancedInputLocalPlayerSubsystem _asbp_player_controller_2) (Variables|Default|GetLeftHandedMappingContext) "(bIgnoreAllPressedKeysUntilRelease=True,bForceImmediately=False,bNotifyUserSettings=False)"))
        (:then_2
          (Input|AddMappingContext (PlayerController|LocalPlayerSubsystems|GetEnhancedInputLocalPlayerSubsystem _asbp_player_controller_2) (Variables|Default|GetRightHandedMappingContext) 0 "(bIgnoreAllPressedKeysUntilRelease=True,bForceImmediately=False,bNotifyUserSettings=False)"))))))

(fn GetSettingsSaveData
  (return (Variables|Default|GetSettingsSaveGame)))

(fn ILoadOtherSettings
  (bind _returnvalue (Class|ELSGameInstance|LoadOtherSettings))
  (return _returnvalue))