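; BP_DoorTest is a puzzle door actor that sinks vertically to open and rises back to close.
; BeginPlay stores the closed Z position.
; The PressurePlate event plays or reverses a timeline, whose track offsets the door below that position by an open depth while keeping X and Y.
; A lookup of the river puzzle manager's pressed-plate event is present but unused.
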(event EventBeginPlay
  ;[0.15 0.15 0.15 0.5] Set default z-position (closed)
  (Variables|Default|SetDefault%20ZPosition (.z (Transformation|GetActorLocation))))

(event EventPressurePlate
  (params (Down? :type Boolean))
  (bind _returnvalue (Transformation|GetActorLocation))
  ;[0.15 0.1413 0.01161 0.502] Open door (play/true) or close door (reverse/false)
  (if Down?
    (bind _down (Timeline|Timeline Play)
      (:Update
        (Transformation|SetActorLocation (Math|Vector|MakeVector (.x _returnvalue) (.y _returnvalue) (- (Variables|Default|GetDefault%20ZPosition) (* _down (Variables|Default|GetOpenDepth)))) false false)))
    (else
      (Timeline|Timeline Reverse))))

(fn ConstructionScript)