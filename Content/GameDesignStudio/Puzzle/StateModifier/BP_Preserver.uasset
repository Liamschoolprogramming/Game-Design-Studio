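; BP_Preserver is a puzzle state modifier that holds the actor in its line of sight in a Preserved state.
; On spawn it plays a stasis beam sound and starts a looping timer that line traces forward, ignoring the player and possessable entities.
; A newly hit actor is set to Preserved through interface messages, and the previous one returns to Default.
; While carried or when deactivated, it releases its target.
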(event Custom|ActivatePreserver
  (params (bActivate :type Boolean))
  ;[0.15 0.15 0.15 0.5] If being carried deactivate and start rotate loop; if on the ground, activate and stop rotate loop
  (if bActivate
    (Utilities|Time|ClearandInvalidateTimerbyHandle (Variables|Default|GetRotateLoop))
    (bind _returnvalue (Utilities|Time|SetTimerbyFunctionName 0 "CheckForTargets" 0.2 true))
    (Variables|Default|SetPreserveLoop _returnvalue)
    (else
      (Utilities|Time|ClearandInvalidateTimerbyHandle (Variables|Default|GetPreserveLoop))
      (Class|BPIPuzzleActivations|ChangePuzzleActorState(Message) (Variables|Default|GetPreservedActor) "Default")
      (Variables|Default|SetPreservedActor 0))))

(event EventBeginPlay
  ;[0.15 0.15 0.15 0.5] Activate preserver as soon as it spawns
  (|CallParentFunction)
  (CallFunction|ActivatePreserver true)
  (Audio|PlaySoundatLocation "/Game/GameDesignStudio/Audio/SFX/Cues/Preserver-Stasis_beam_sfx_Cue.Preserver-Stasis_beam_sfx_Cue" (Transformation|GetActorLocation) "0, 0, 0" 1.0 1.0 0.0 0 0 0 0))

(fn ConstructionScript)

(fn CheckforTargets
  (bind _cylinder (Variables|Default|GetCylinder))
  (bind _returnvalue (Transformation|GetWorldLocation _cylinder))
  ;[0.15 0.15 0.15 0.5] If line trace hits an object, it tries to preserve its state by calling the BPI; If the preserver loses sight of the object, it calls the BPI to return the object to default state
  (if (Variables|Default|GetbBeingCarried)
    (bind _preservedactor (Variables|Default|GetPreservedActor)
      (:then
        (Class|BPIPuzzleActivations|ChangePuzzleActorState(Message) _preservedactor "Default")
        (Variables|Default|SetPreservedActor 0))
      (:else))
    (else
      (bind _outactors (Actor|GetAllActorsOfClass "/Game/GameDesignStudio/Possessables/BP_PossessableEntity.BP_PossessableEntity_C"))
      (Variables|Default|SetActorsToIgnore _outactors)
      (bind _returnvalue_2 (Actor|GetActorOfClass "/Game/GameDesignStudio/Characters/BP_PlayerCharacter.BP_PlayerCharacter_C"))
      (Utilities|Array|Add (Variables|Default|GetActorsToIgnore) _returnvalue_2)
      (bind (_outhit _returnvalue_3) (Collision|LineTraceByChannel _returnvalue (+ _returnvalue (* (Math|Vector|GetForwardVector (Variables|Default|GetCube)) 5e+03)) "TraceTypeQuery3" false (Variables|Default|GetActorsToIgnore) "ForDuration" true "(R=1.000000,G=0.000000,B=0.000000,A=1.000000)" "(R=0.000000,G=1.000000,B=0.000000,A=1.000000)" 0.2))
      (if _returnvalue_3
        _
        (else
          (Variables|Default|SetbHasActivatingElement false)))
      (LocalVariables|SetL_NewActor (.HitActor (Collision|BreakHitResult _outhit)))
      (bind _preservedactor_2 (Variables|Default|GetPreservedActor)
        (:then
          (if (not (== _preservedactor_2 (LocalVariables|GetL_NewActor)))
            (Class|BPIPuzzleActivations|ChangePuzzleActorState(Message) (Variables|Default|GetPreservedActor) "Default")
            (Variables|Default|SetbHasActivatingElement false)
            (bind _epuzzlestate (Class|BPIPuzzleActivations|CheckPuzzleActorState(Message) (LocalVariables|GetL_NewActor)))
            (switch Utilities|FlowControl|Switch|SwitchonEPuzzleElementState _epuzzlestate
              (:Default
                (bind _output_get (Variables|Default|SetPreservedActor (LocalVariables|GetL_NewActor)))
                (Class|BPIPuzzleActivations|ChangePuzzleActorState(Message) _output_get "Preserved")
                (Variables|Default|SetbHasActivatingElement true)))))
        (:else
          (bind _epuzzlestate_2 (Class|BPIPuzzleActivations|CheckPuzzleActorState(Message) (LocalVariables|GetL_NewActor)))
          (switch Utilities|FlowControl|Switch|SwitchonEPuzzleElementState _epuzzlestate_2
            (:Default
              (bind _output_get_2 (Variables|Default|SetPreservedActor (LocalVariables|GetL_NewActor)))
              (Class|BPIPuzzleActivations|ChangePuzzleActorState(Message) _output_get_2 "Preserved")
              (Variables|Default|SetbHasActivatingElement true))))))))