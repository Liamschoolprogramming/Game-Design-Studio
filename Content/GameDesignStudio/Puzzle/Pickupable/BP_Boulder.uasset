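; BP_Boulder is a pickupable puzzle object that snaps onto pressure plates and flower platforms.
; When its Cube hits a pressure plate or a flower platform's Platform component, it moves just above that target, skipping the move if X already matches.
; On flower platforms it also attaches to the Platform, keeping world transform.
; Pickup attachment defers to the parent class, while the collision toggle extends the parent's to switch its Box.
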(event OnComponentHit(Cube)
  (params (HitComponent :type Primitive%20Component%20Object%20Reference) (OtherActor :type Actor%20Object%20Reference) (OtherComp :type Primitive%20Component%20Object%20Reference) (NormalImpulse :type Vector :default "0, 0, 0") (Hit :type Hit%20Result%20Structure%20%28by%20ref%29))
  (bind _hitactor (Collision|BreakHitResult Hit))
  ;[0.15 0.15 0.15 0.5] Disables physics and resets rotation when object hits the ground; if lands on pressure plant, snaps to center of pressure plant
  (CallFunction|SnaptoPressurePlant _hitactor)
  (CallFunction|SnaptoFlowerPlatform _hitactor))

(event EventAttachPickupAble
  (params (Attach :type Boolean))
  (|CallParentFunction Attach))

(event EventBeginPlay
  (|CallParentFunction))

(fn ConstructionScript)

(fn SnaptoPressurePlant
  (params (HitActor :type Actor%20Object%20Reference))
  (if (Class|GameplayStatics|ObjectIsA HitActor "/Game/GameDesignStudio/Puzzle/PressurePlate/BP_PressurePlate.BP_PressurePlate_C")
    (bind _output_get (LocalVariables|SetL_PressurePlantLocation (Transformation|GetActorLocation HitActor)))
    (if (!= (.x _output_get) (.x (Transformation|GetActorLocation)))
      (Transformation|SetActorLocation (Math|Vector|MakeVector (.x (LocalVariables|GetL_PressurePlantLocation)) (.y (LocalVariables|GetL_PressurePlantLocation)) (+ (.z (LocalVariables|GetL_PressurePlantLocation)) 1e+01)) false false))))

(fn CollisionToggle
  (params (ToggleOn :type Boolean))
  (|CallParentFunction ToggleOn)
  (if ToggleOn
    (Collision|SetCollisionEnabled (Variables|Default|GetBox) "QueryAndPhysics")
    (else
      (Collision|SetCollisionEnabled (Variables|Default|GetBox) "NoCollision"))))

(fn SnaptoFlowerPlatform
  (params (HitActor :type Actor%20Object%20Reference))
  (if (Class|GameplayStatics|ObjectIsA HitActor "/Game/GameDesignStudio/Puzzle/FlowerPlatform/BP_FlowerPlatform.BP_FlowerPlatform_C")
    (bind _asbp_flower_platform (Utilities|Casting|CastToBP_FlowerPlatform HitActor))
    (bind _output_get (LocalVariables|SetPlatform (Variables|/Game/GameDesignStudio/Puzzle/FlowerPlatform/BP_FlowerPlatform.BP_FlowerPlatform_C|GetPlatform _asbp_flower_platform)))
    (bind _output_get_2 (LocalVariables|SetPlatformLocation (Transformation|GetWorldLocation _output_get)))
    (if (!= (.x _output_get_2) (.x (Transformation|GetActorLocation)))
      (Transformation|SetActorLocation (Math|Vector|MakeVector (.x (LocalVariables|GetPlatformLocation)) (.y (LocalVariables|GetPlatformLocation)) (+ (.z (LocalVariables|GetPlatformLocation)) 1e+01)) false false)
      (Transformation|AttachComponentToComponent self (LocalVariables|GetPlatform) "None" "KeepWorld" "KeepWorld" "KeepWorld" true))))