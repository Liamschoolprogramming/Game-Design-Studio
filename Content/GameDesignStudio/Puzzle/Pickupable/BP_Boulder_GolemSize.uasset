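; BP_Boulder_GolemSize is a pickupable puzzle boulder that can rest on pressure plates.
; Click, attach and BeginPlay behavior pass through to its parent class.
; When its cube hits a mostly upward-facing surface, it stops simulating physics, resets rotation to yaw only and restarts the range-check loop.
; Landing on a BP_PressurePlate snaps it to the plate's XY center while keeping its height, but only if their X positions differ.
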(event OnComponentHit(Cube)
  (params (HitComponent :type Primitive%20Component%20Object%20Reference) (OtherActor :type Actor%20Object%20Reference) (OtherComp :type Primitive%20Component%20Object%20Reference) (NormalImpulse :type Vector :default "0, 0, 0") (Hit :type Hit%20Result%20Structure%20%28by%20ref%29))
  (bind (_bblockinghit _binitialoverlap _time _distance _location _impactpoint _normal _impactnormal _physmat _hitactor) (Collision|BreakHitResult Hit))
  ;[0.15 0.15 0.15 0.5] Disables physics and resets rotation when object hits the ground; if lands on pressure plant, snaps to center of pressure plant
  (if (>= (.Z (Math|Vector|BreakVector _normal)) 0.7)
    (Physics|SetSimulatePhysics (Variables|Default|GetCube) false)
    (Transformation|SetActorRotation (Math|Rotator|MakeRotator 0.0 0.0 (.yaw (Transformation|GetActorRotation))))
    (CallFunction|SnaptoPressurePlant _hitactor)
    (CallFunction|RunCheckforRangeLoop true)))

(event EventAttachPickupAble
  (params (Attach :type Boolean))
  (|CallParentFunction Attach))

(event MouseInput|EventActorOnClicked
  (params (ButtonPressed :type Key%20Structure))
  (|CallParentFunction ButtonPressed))

(event EventBeginPlay
  (|CallParentFunction))

(fn ConstructionScript)

(fn SnaptoPressurePlant
  (params (HitActor :type Actor%20Object%20Reference))
  (if (Class|GameplayStatics|ObjectIsA HitActor "/Game/GameDesignStudio/Puzzle/PressurePlate/BP_PressurePlate.BP_PressurePlate_C")
    (bind _output_get (LocalVariables|SetL_PressurePlantLocation (Transformation|GetActorLocation HitActor)))
    (if (!= (.x _output_get) (.x (Transformation|GetActorLocation)))
      (Transformation|SetActorLocation (Math|Vector|MakeVector (.x (LocalVariables|GetL_PressurePlantLocation)) (.y (LocalVariables|GetL_PressurePlantLocation)) (.z (Transformation|GetActorLocation))) false false))))