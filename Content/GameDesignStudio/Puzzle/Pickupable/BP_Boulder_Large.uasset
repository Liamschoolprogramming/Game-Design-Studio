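; Large boulder interactable that, once successfully interacted with, slides itself along world +Y to a set destination.
; OnInteract refuses players standing in an item gate, otherwise calls Interact and prints the character type as debug text.
; The first time this leaves it flagged as carried, a one-shot flag starts a fast looping timer.
; Each tick nudges the boulder without sweeping until it passes PushDestination, then clears the timer.
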(event Custom|PushBoulder
  (Transformation|SetActorLocation (+ (Transformation|GetActorLocation) "0.000000,5.000000,0.000000") false false)
  (if (>= (.y (Transformation|GetActorLocation)) (Variables|Default|GetPushDestination))
    (Utilities|Time|ClearandInvalidateTimerbyHandle (Variables|Default|GetPushTimer))))

(event MouseInput|EventActorOnClicked
  (params (ButtonPressed :type Key%20Structure :default "None")))

(event EventOnInteract
  (params (PlayerCharacter :type Player%20Character%20Object%20Reference))
  (bind _asplayer_character (Utilities|Casting|CastToPlayerCharacter PlayerCharacter))
  (if (Variables|/Script/GameDesignStudio.PlayerCharacter|GetbIsInItemGate _asplayer_character)
    (Development|PrintString "can't pick up")
    (else
      (Class|PuzzleInteractivePickupable|Interact self _asplayer_character)
      (Development|PrintString (Utilities|String|EnumtoString (Variables|/Script/GameDesignStudio.PlayerCharacter|GetPlayerCharacterType _asplayer_character)) true true "(R=1.000000,G=0.783057,B=0.000000,A=1.000000)")
      (if (not (Variables|Default|GetBoulderPushed))
        (if (Variables|Default|GetbBeingCarried)
          (Variables|Default|SetBoulderPushed true)
          (bind _returnvalue (Utilities|Time|SetTimerbyEvent (delegate Custom|PushBoulder) 0.01 true))
          (Variables|Default|SetPushTimer _returnvalue))))))

(fn ConstructionScript)