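; Puzzle pickupable actor that the player can carry and drop, showing an indicator FX and prompt billboard when within interact range.
; A looping timer checks player distance against the InteractRange stat while the object is available.
; AttachPickupAble disables physics and snaps it to the player's Socket_Carry, or detaches it to fall.
; Hitting a floor-like surface stops physics, resets rotation keeping yaw, and restarts the range check.
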(event OnComponentHit(Cube)
  (params (HitComponent :type Primitive%20Component%20Object%20Reference) (OtherActor :type Actor%20Object%20Reference) (OtherComp :type Primitive%20Component%20Object%20Reference) (NormalImpulse :type Vector :default "0, 0, 0") (Hit :type Hit%20Result%20Structure%20%28by%20ref%29))
  ;[0.15 0.15 0.15 0.5] Disables physics and resets rotation when object hits the ground; if lands on pressure plant, snaps to center of pressure plant
  (if (>= (.Z (Math|Vector|BreakVector (.Normal (Collision|BreakHitResult Hit)))) 0.7)
    (Physics|SetSimulatePhysics (Variables|Default|GetCube) false)
    (Transformation|SetActorRotation (Math|Rotator|MakeRotator 0.0 0.0 (.yaw (Transformation|GetActorRotation))))
    (CallFunction|RunCheckforRangeLoop true)))

(event MouseInput|EventActorOnClicked
  (params (ButtonPressed :type Key%20Structure :default "None"))
  (bind _asplayer_character (Utilities|Casting|CastToPlayerCharacter (Game|GetPlayerCharacter 0)))
  (if (not (Variables|/Script/GameDesignStudio.PlayerCharacter|GetbIsInItemGate _asplayer_character))
    (Class|PuzzleInteractivePickupable|Interact self _asplayer_character)))

(event EventAttachPickupAble
  (params (Attach :type Boolean))
  (bind _returnvalue (Game|GetPlayerCharacter 0))
  (bind _mesh (Variables|/Script/Engine.Character|GetMesh _returnvalue))
  (bind _returnvalue_2 (Transformation|GetSocketLocation _mesh "Socket_Carry"))
  ;[0.15 0.15 0.15 0.5] When picked up, disables physics and attaches actor to player; when dropped, detaches from player and enables physics so it can fall
  (if Attach
    (Physics|SetSimulatePhysics (Variables|Default|GetCube) false)
    (CallFunction|CollisionToggle false)
    (bind _asbp_player_character (Utilities|Casting|CastToBP_PlayerCharacter _returnvalue)
      (:then
        (Transformation|SetActorLocation (Transformation|GetSocketLocation (Variables|/Game/GameDesignStudio/Characters/BP_PlayerCharacter.BP_PlayerCharacter_C|GetStaticMesh_TPP _asbp_player_character) "Socket_Carry") false true)
        (Transformation|SetActorRotation (Transformation|GetWorldRotation (Variables|/Script/Engine.Actor|GetRootComponent (Game|GetPlayerCharacter 0))))
        (Transformation|AttachComponentToComponent (Variables|/Game/GameDesignStudio/Characters/BP_PlayerCharacter.BP_PlayerCharacter_C|GetStaticMesh_TPP _asbp_player_character) "Socket_Carry" "SnapToTarget" "KeepWorld" "KeepWorld" true)
        (CallFunction|RunCheckforRangeLoop false))
      (:CastFailed
        (Transformation|SetActorLocation (Math|Vector|MakeVector (.x _returnvalue_2) (.y _returnvalue_2) (.z _returnvalue_2)) false true)
        (Transformation|SetActorRotation (Transformation|GetWorldRotation (Variables|/Script/Engine.Actor|GetRootComponent (Game|GetPlayerCharacter 0))))
        (Transformation|AttachComponentToComponent (Variables|/Script/Engine.Character|GetMesh (Game|GetPlayerCharacter 0)) "Socket_Carry" "KeepWorld" "KeepWorld" "KeepWorld" true)
        (CallFunction|RunCheckforRangeLoop false)))
    (else
      (Transformation|DetachFromActor "KeepWorld" "KeepWorld" "KeepWorld")
      (Physics|SetSimulatePhysics (Variables|Default|GetCube) true)
      (CallFunction|CollisionToggle true))))

(event EventBeginPlay
  (CallFunction|RunCheckforRangeLoop true))

(fn ConstructionScript)

(fn RunCheckforRangeLoop
  (params (RunLoop? :type Boolean))
  ;[0.15 0.15 0.15 0.5] Run the loop to check if player is in range to pickup and display the indicator
  (if RunLoop?
    (if (not (Utilities|Time|IsTimerActivebyHandle (Variables|Default|GetPickupRangeTimer)))
      (bind _returnvalue (Utilities|Time|SetTimerbyFunctionName 0 "CheckWithinPickupRange" 0.05 true))
      (Variables|Default|SetPickupRangeTimer _returnvalue))
    (else
      (Components|Activation|Deactivate (Variables|Default|GetPickupIndicatorFX))
      (Rendering|SetVisibility (Variables|Default|GetBillboard) false false)
      (Utilities|Time|ClearandInvalidateTimerbyHandle (Variables|Default|GetPickupRangeTimer)))))

(fn CheckWithinPickupRange
  ;[0.15 0.15 0.15 0.5] If the player is in the interact range, show FX and Press E prompt; Otherwise, disable the FX and don't show the prompt
  (bind _returnvalue (Class|PlayerStatManager|GetPlayerStats (Class|GameManagerSubsystem|GetPlayerStatManager (Subsystems|GetGameManagerSubsystem))))
  (LocalVariables|SetL_InteractRange (.InteractRange (Utilities|Struct|BreakPlayerStats _returnvalue)))
  (if (<= (Transformation|GetDistanceTo self (Game|Player|GetPlayerPawn 0)) (LocalVariables|GetL_InteractRange))
    (Rendering|SetVisibility (Variables|Default|GetBillboard) true false)
    (if (not (Components|Activation|IsActive (Variables|Default|GetPickupIndicatorFX)))
      (Components|Activation|Activate (Variables|Default|GetPickupIndicatorFX) false))
    (else
      (Rendering|SetVisibility (Variables|Default|GetBillboard) false false)
      (if (Components|Activation|IsActive (Variables|Default|GetPickupIndicatorFX))
        (Components|Activation|Deactivate (Variables|Default|GetPickupIndicatorFX))))))

(fn CollisionToggle
  (params (ToggleOn :type Boolean))
  (if ToggleOn
    (Collision|SetCollisionEnabled (Variables|Default|GetCube) "QueryAndPhysics")
    (else
      (Collision|SetCollisionEnabled (Variables|Default|GetCube) "ProbeOnly"))))