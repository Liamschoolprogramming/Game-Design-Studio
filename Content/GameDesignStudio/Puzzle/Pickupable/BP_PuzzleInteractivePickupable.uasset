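; Puzzle pickup object that the player clicks to interact with, refused while in an item gate, and carries on the character's Socket_Carry.
; AttachPickupAble toggles the cube's physics and collision as it attaches or detaches.
; A hit on a floor-like surface stops physics, keeps only yaw and restarts the range check.
; That looping timer swaps the cube's material when the player is within the interact range from player stats.
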(event OnComponentHit(Cube)
  (params (HitComponent :type Primitive%20Component%20Object%20Reference) (OtherActor :type Actor%20Object%20Reference) (OtherComp :type Primitive%20Component%20Object%20Reference) (NormalImpulse :type Vector :default "0, 0, 0") (Hit :type Hit%20Result%20Structure%20%28by%20ref%29))
  ;[0.15 0.15 0.15 0.5] Disables physics and resets rotation when object hits the ground; if lands on pressure plant, snaps to center of pressure plant
  (if (>= (.Z (Math|Vector|BreakVector (.Normal (Collision|BreakHitResult Hit)))) 0.7)
    (Physics|SetSimulatePhysics (Variables|Default|GetCube) false)
    (Transformation|SetActorRotation (Math|Rotator|MakeRotator 0.0 0.0 (.yaw (Transformation|GetActorRotation))))
    (CallFunction|RunCheckforRangeLoop true)))

(event MouseInput|EventActorOnClicked
  (params (ButtonPressed :type Key%20Structure :default "None"))
  (bind _asplayer_character (Utilities|Casting|CastToPlayerCharacter (Game|GetPlayerCharacter 0)))
  (if (Variables|/Script/GameDesignStudio.PlayerCharacter|GetbIsInItemGate _asplayer_character)
    (Development|PrintString "can't pick up")
    (else
      (Class|PuzzleInteractivePickupable|Interact self _asplayer_character))))

(event EventAttachPickupAble
  (params (Attach :type Boolean))
  (bind _returnvalue (Game|GetPlayerCharacter 0))
  (bind _mesh (Variables|/Script/Engine.Character|GetMesh _returnvalue))
  ;[0.15 0.15 0.15 0.5] When picked up, disables physics and attaches actor to player; when dropped, detaches from player and enables physics so it can fall
  (if Attach
    (Physics|SetSimulatePhysics (Variables|Default|GetCube) false)
    (Collision|SetCollisionEnabled (Variables|Default|GetCube) "NoCollision")
    (Transformation|SetActorLocation (Transformation|GetSocketLocation (Components|GetChildComponent _mesh 0) "Socket_Carry") false true)
    (Transformation|SetActorRotation (Transformation|GetWorldRotation (Variables|/Script/Engine.Actor|GetRootComponent (Game|GetPlayerCharacter 0))))
    (Transformation|AttachComponentToComponent _mesh "Socket_Carry" "KeepWorld" "KeepWorld" "KeepWorld" true)
    (CallFunction|RunCheckforRangeLoop false)
    (else
      (Transformation|DetachFromActor "KeepWorld" "KeepWorld" "KeepWorld")
      (Physics|SetSimulatePhysics (Variables|Default|GetCube) true)
      (Collision|SetCollisionEnabled (Variables|Default|GetCube) "QueryAndPhysics"))))

(event EventBeginPlay
  (CallFunction|RunCheckforRangeLoop true))

(fn ConstructionScript)

(fn RunCheckforRangeLoop
  (params (RunLoop? :type Boolean))
  ;[0.15 0.15 0.15 0.5] Run the loop to check if player is in range to pickup and display the indicator
  (if RunLoop?
    (if (not (Utilities|Time|IsTimerActivebyHandle (Variables|Default|GetPickupRangeTimer)))
      (bind _returnvalue (Utilities|Time|SetTimerbyFunctionName 0 "CheckWithinPickupRange" 0.5 true))
      (Variables|Default|SetPickupRangeTimer _returnvalue))
    (else
      (Rendering|Material|SetMaterial (Variables|Default|GetCube) 0 "/Game/GameDesignStudio/MaterialLibrary/CelShader/MI_Cel_Ex3.MI_Cel_Ex3")
      (Utilities|Time|ClearandInvalidateTimerbyHandle (Variables|Default|GetPickupRangeTimer)))))

(fn CheckWithinPickupRange
  (bind _returnvalue (Class|PlayerStatManager|GetPlayerStats (Class|GameManagerSubsystem|GetPlayerStatManager (Subsystems|GetGameManagerSubsystem))))
  (LocalVariables|SetL_InteractRange (.InteractRange (Utilities|Struct|BreakPlayerStats _returnvalue)))
  (if (<= (Transformation|GetDistanceTo self (Game|Player|GetPlayerPawn 0)) (LocalVariables|GetL_InteractRange))
    (bind _output_get (LocalVariables|SetL_Material (Rendering|Material|GetMaterial (Variables|Default|GetCube) 0)))
    (if (== _output_get "/Game/GameDesignStudio/MaterialLibrary/CelShader/MI_Cel_Ex3.MI_Cel_Ex3")
      (Rendering|Material|SetMaterial (Variables|Default|GetCube) 0 "/Game/GameDesignStudio/MaterialLibrary/CelShader/MI_Cel_Ex1.MI_Cel_Ex1"))
    (else
      (bind _output_get_2 (LocalVariables|SetL_Material (Rendering|Material|GetMaterial (Variables|Default|GetCube) 0)))
      (if (not (== _output_get_2 "/Game/GameDesignStudio/MaterialLibrary/CelShader/MI_Cel_Ex3.MI_Cel_Ex3"))
        (Rendering|Material|SetMaterial (Variables|Default|GetCube) 0 "/Game/GameDesignStudio/MaterialLibrary/CelShader/MI_Cel_Ex3.MI_Cel_Ex3")))))