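; Pushable puzzle boulder that the player attaches to and moves by walking, with an interact-range indicator and prompt.
; Attaching enables physics, turns and spaces the player, changes movement speed, and passes push state and axis to the player controller.
; A fast looping timer then offsets the boulder along player facing to hold a fixed gap until detach.
; Range polling targets CheckWithinPickupRange by name, while the function here is CheckWithinPushRange.
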(event OnComponentBeginOverlap(PushTrigger)
  (params (OverlappedComponent :type Primitive%20Component%20Object%20Reference) (OtherActor :type Actor%20Object%20Reference) (OtherComp :type Primitive%20Component%20Object%20Reference) (OtherBodyIndex :type Integer) (bFromSweep :type Boolean) (SweepResult :type Hit%20Result%20Structure%20%28by%20ref%29))
  (Variables|Default|SetbIsInPushRange true))

(event OnComponentEndOverlap(PushTrigger)
  (params (OverlappedComponent :type Primitive%20Component%20Object%20Reference) (OtherActor :type Actor%20Object%20Reference) (OtherComp :type Primitive%20Component%20Object%20Reference) (OtherBodyIndex :type Integer))
  (Variables|Default|SetbIsInPushRange false))

(event EventAttachPickupAble
  (params (Attach :type Boolean))
  (bind _returnvalue (Game|GetPlayerCharacter 0))
  (bind _returnvalue_2 (Transformation|GetActorRotation _returnvalue))
  (bind _returnvalue_3 (Math|Vector|GetForwardVector _returnvalue_2))
  (if Attach
    (Physics|SetSimulatePhysics (Variables|Default|GetCube) true)
    (bind _bp_player_controller (Class|BPIPlayerControllerPossession|GetBPPlayerController(Message) (Game|GetPlayerController 0)))
    (Variables|/Script/GameDesignStudio.PlayerControllerBase|SetPawnMovementSpeed _bp_player_controller 3e+02)
    (Transformation|SetActorRotation (Game|GetPlayerCharacter 0) (Math|Interpolation|RInterpTo (Transformation|GetActorRotation (Game|GetPlayerCharacter 0)) (Math|Rotator|FindLookatRotation (Transformation|GetActorLocation (Game|GetPlayerCharacter 0)) (Transformation|GetActorLocation)) 1.0 1.0))
    (if (<= (Math|Vector|Distance(Vector) (Transformation|GetActorLocation (Game|GetPlayerCharacter 0)) (Transformation|GetActorLocation)) 4.8e+02)
      (Transformation|SetActorLocation (Game|GetPlayerCharacter 0) (+ (Transformation|GetActorLocation (Game|GetPlayerCharacter 0)) (* (Math|Vector|MakeVector (.x _returnvalue_3) (.y _returnvalue_3) 0.0) -1e+02)) true false))
    (Variables|/Script/GameDesignStudio.PlayerControllerBase|SetBoulderPushForwardAxis _bp_player_controller (Math|Vector|GetForwardVector (Transformation|GetActorRotation (Game|GetPlayerCharacter 0))))
    (Variables|/Script/GameDesignStudio.PlayerControllerBase|SetbIsPushingBoulder _bp_player_controller true)
    (bind _returnvalue_4 (Utilities|Time|SetTimerbyFunctionName 0 "PushBoulder" 0.01 true))
    (Variables|Default|SetPushTimer _returnvalue_4)
    (else
      (Physics|SetSimulatePhysics (Variables|Default|GetCube) false)
      (bind _bp_player_controller_2 (Class|BPIPlayerControllerPossession|GetBPPlayerController(Message) (Game|GetPlayerController 0)))
      (Variables|/Script/GameDesignStudio.PlayerControllerBase|SetPawnMovementSpeed _bp_player_controller_2 4e+02)
      (Variables|/Script/GameDesignStudio.PlayerControllerBase|SetbIsPushingBoulder _bp_player_controller_2 false)
      (Utilities|Time|ClearandInvalidateTimerbyHandle (Variables|Default|GetPushTimer)))))

(event EventBeginPlay
  (CallFunction|RunCheckforRangeLoop true))

(fn ConstructionScript)

(fn RunCheckforRangeLoop
  (params (RunLoop? :type Boolean))
  ;[0.15 0.15 0.15 0.5] Run the loop to check if player is in range to pickup and display the indicator
  (if RunLoop?
    (if (not (Utilities|Time|IsTimerActivebyHandle (Variables|Default|GetPickupRangeTimer)))
      (bind _returnvalue (Utilities|Time|SetTimerbyFunctionName 0 "CheckWithinPickupRange" 0.05 true))
      (Variables|Default|SetPickupRangeTimer _returnvalue))
    (else
      (Components|Activation|Deactivate (Variables|Default|GetPickupIndicatorFX))
      (Rendering|SetVisibility (Variables|Default|GetBillboard) false false)
      (Utilities|Time|ClearandInvalidateTimerbyHandle (Variables|Default|GetPickupRangeTimer)))))

(fn CheckWithinPushRange
  ;[0.15 0.15 0.15 0.5] If the player is in the interact range, show FX and Press E prompt; Otherwise, disable the FX and don't show the prompt
  (bind _returnvalue (Class|PlayerStatManager|GetPlayerStats (Class|GameManagerSubsystem|GetPlayerStatManager (Subsystems|GetGameManagerSubsystem))))
  (LocalVariables|SetL_InteractRange (.InteractRange (Utilities|Struct|BreakPlayerStats _returnvalue)))
  (if (<= (Transformation|GetDistanceTo self (Game|Player|GetPlayerPawn 0)) (LocalVariables|GetL_InteractRange))
    (Rendering|SetVisibility (Variables|Default|GetBillboard) true false)
    (if (not (Components|Activation|IsActive (Variables|Default|GetPickupIndicatorFX)))
      (Components|Activation|Activate (Variables|Default|GetPickupIndicatorFX) false))
    (else
      (Rendering|SetVisibility (Variables|Default|GetBillboard) false false)
      (if (Components|Activation|IsActive (Variables|Default|GetPickupIndicatorFX))
        (Components|Activation|Deactivate (Variables|Default|GetPickupIndicatorFX))))))

(fn PushBoulder
  (bind _returnvalue (Game|GetPlayerCharacter 0))
  (bind _returnvalue_2 (Transformation|GetActorRotation _returnvalue))
  (bind _returnvalue_3 (Math|Vector|GetForwardVector _returnvalue_2))
  (Transformation|SetActorLocation (+ (Transformation|GetActorLocation) (* (Math|Vector|MakeVector (.x _returnvalue_3) (.y _returnvalue_3) 0.0) (- 5e+02 (Math|Vector|Distance(Vector) (Transformation|GetActorLocation (Game|GetPlayerCharacter 0)) (Transformation|GetActorLocation))))) false false))