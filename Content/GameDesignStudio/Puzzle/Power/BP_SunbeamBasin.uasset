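; Sunbeam basin puzzle piece that relays a powered or unpowered state to its linked puzzle receiver.
; Green and red signals each swap the cylinder material and forward the signal with the puzzle GUID, and red also clears the light timer.
; Shortly after BeginPlay it fills an ignore list with all possessable entities and the player pawn.
; Handling of multiple light sources is still a TODO.
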(event EventGreenSignal
  (params (EmitterId :type Guid%20Structure))
  (Rendering|Material|SetMaterial (Variables|Default|GetCylinder) 0 "/Game/GameDesignStudio/MaterialLibrary/CelShader/MI_Cel_Ex2.MI_Cel_Ex2")
  (bind _aspuzzle_receiver (Utilities|Casting|CastToPuzzleReceiver (Variables|Default|GetLinkedReceiver)))
  (Class|PuzzleReceiver|ReceiveGreenSignal _aspuzzle_receiver (Variables|Default|GetPuzzleActorGuid)))

(event EventRedSignal
  (params (EmitterId :type Guid%20Structure))
  ;[0.15 0.15 0.15 0.5] TODO handle multiple light sources
  (Rendering|Material|SetMaterial (Variables|Default|GetCylinder) 0 "/Game/GameDesignStudio/MaterialLibrary/CelShader/MI_Cel_Global.MI_Cel_Global")
  (Utilities|Time|ClearandInvalidateTimerbyHandle (Variables|Default|GetLightTimer))
  (bind _aspuzzle_receiver (Utilities|Casting|CastToPuzzleReceiver (Variables|Default|GetLinkedReceiver)))
  (Class|PuzzleReceiver|ReceiveRedSignal _aspuzzle_receiver (Variables|Default|GetPuzzleActorGuid)))

(event EventBeginPlay
  (|CallParentFunction)
  (Utilities|FlowControl|Delay 0.2)
  (bind _outactors (Actor|GetAllActorsOfClass "/Script/GameDesignStudio.PossessableEntity"))
  (bind _output_get (Variables|Default|SetIgnoreActors _outactors))
  (Utilities|Array|Add _output_get (Game|Player|GetPlayerPawn 0)))

(fn ConstructionScript)