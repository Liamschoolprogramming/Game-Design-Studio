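; Light puzzle prism that, once lit through RefractLight, emits a Niagara beam along its arrow and passes light on to other prisms or sunbeam basins.
; A looping timer runs a line trace that ignores the player and possessable entities, with reach scaled by horizontal distance to the light source.
; Hit basins get a green signal keyed by the prism's GUID, and a red one when the trace loses them.
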(event EventBeginPlay
  (Niagara|SetNiagaraVariable(Float) (Variables|Default|GetLightBeam) "ScaleAlpha" 0.0)
  (Utilities|FlowControl|Delay 0.2)
  (bind _outactors (Actor|GetAllActorsOfClass "/Script/GameDesignStudio.PossessableEntity"))
  (bind _output_get (Variables|Default|SetIgnore%20Actors _outactors))
  (Utilities|Array|Add _output_get (Game|Player|GetPlayerPawn 0)))

(fn ConstructionScript
  (Variables|Default|SetPrismGuid (Guid|NewGuid)))

(fn LightTrace
  (bind _destination (CallFunction|GetDestinationPoint))
  (LocalVariables|SetL_Destination _destination)
  (bind (_outhit _returnvalue) (Collision|LineTraceByChannel (Transformation|GetActorLocation) (LocalVariables|GetL_Destination) "TraceTypeQuery1" false (Variables|Default|GetIgnore%20Actors) "None" true "(R=0.477561,G=0.008604,B=1.000000,A=1.000000)" "(R=0.000000,G=1.000000,B=0.000000,A=1.000000)" 1.0))
  (LocalVariables|SetL_HitSomething _returnvalue)
  (LocalVariables|SetL_HitActor (.HitActor (Collision|BreakHitResult _outhit)))
  (if (LocalVariables|GetL_HitSomething)
    (Utilities|IsValid (Variables|Default|GetReceivingLightActor)
      (:Is%20Valid
        (if (!= (Variables|Default|GetReceivingLightActor) (LocalVariables|GetL_HitActor))
          (CallFunction|ClearReceivingActor)))
      (:Is%20Not%20Valid
        (bind _output_get (Variables|Default|SetReceivingLightActor (LocalVariables|GetL_HitActor)))
        (bind _asbp_sunbeam_basin (Utilities|Casting|CastToBP_SunbeamBasin _output_get)
          (:then
            (Class|PuzzleReceiver|ReceiveGreenSignal _asbp_sunbeam_basin (Variables|Default|GetPrismGuid)))
          (:CastFailed
            (bind _output_get_2 (Variables|Default|SetReceivingLightActor (LocalVariables|GetL_HitActor)))
            (bind _asbp_refracting_prism (Utilities|Casting|CastToBP_RefractingPrism _output_get_2))
            (bind _output_get_3 (Variables|Default|SetReceivingLightActor _asbp_refracting_prism))
            (CallFunction|RefractLight _output_get_3)))))
    (else
      (CallFunction|ClearReceivingActor))))

(fn RefractLight
  (params (LightSource :type Actor%20Object%20Reference))
  (Variables|Default|SetLightSourceActor LightSource)
  (bind _destination (CallFunction|GetDestinationPoint))
  (Components|Activation|SetActive (Variables|Default|GetLightBeam) true false)
  (Transformation|SetWorldRotation (Variables|Default|GetLightBeam) (Math|Rotator|MakeRotator 0.0 -9e+01 (.yaw (Math|Rotator|FindLookatRotation (Transformation|GetActorLocation) _destination))) false false)
  (Components|Activation|Activate (Variables|Default|GetLightBeam) false)
  (bind _returnvalue (Utilities|Time|SetTimerbyFunctionName 0 "LightTrace" 0.05 true))
  (Variables|Default|SetLightTraceTimer _returnvalue))

(fn GetDestinationPoint
  (bind _range (Variables|Default|GetRange))
  (bind _lightsourceactor (Variables|Default|GetLightSourceActor))
  (bind _returnvalue (Transformation|GetHorizontalDistanceTo _lightsourceactor))
  (bind _returnvalue_2 (* _returnvalue _range))
  (return (+ (Transformation|GetActorLocation) (* (Math|Vector|MakeVector _returnvalue_2 _returnvalue_2 _returnvalue_2) (Math|Vector|GetForwardVector (Variables|Default|GetArrow))))))

(fn ClearReceivingActor
  (bind _asbp_sunbeam_basin (Utilities|Casting|CastToBP_SunbeamBasin (Variables|Default|GetReceivingLightActor))
    (:then
      (Class|PuzzleReceiver|ReceiveRedSignal _asbp_sunbeam_basin (Variables|Default|GetPrismGuid)))
    (:CastFailed
      _))
  (Variables|Default|SetReceivingLightActor 0))

(fn SetLightBeamDestination
  (bind _destination (CallFunction|GetDestinationPoint))
  (Class|NiagaraComponent|SetNiagaraVariableVec3 (Variables|Default|GetLightBeam) "BeamEnd" _destination))

(fn StopLight
  (Components|Activation|SetActive (Variables|Default|GetLightBeam) false false)
  (Utilities|Time|ClearandInvalidateTimerbyHandle (Variables|Default|GetLightTraceTimer))
  (Variables|Default|SetLightSourceActor 0)
  (bind _asbp_sunbeam_basin (Utilities|Casting|CastToBP_SunbeamBasin (Variables|Default|GetReceivingLightActor)))
  (Class|PuzzleReceiver|ReceiveRedSignal _asbp_sunbeam_basin (Variables|Default|GetPrismGuid)))