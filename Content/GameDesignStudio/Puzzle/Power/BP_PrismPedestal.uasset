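; Puzzle pedestal holding a refracting prism that can be rotated to redirect a light beam.
; RotatePrism turns input into frame-rate-scaled rotation of the prism child actor, with free yaw and tightly clamped pitch.
; After each rotation it has the BP_RefractingPrism recompute its beam destination.
; Click and pickup-attach behavior defers entirely to the parent class.
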(event EventBeginPlay
  (|CallParentFunction))

(event MouseInput|EventActorOnClicked
  (params (ButtonPressed :type Key%20Structure :default "None"))
  (|CallParentFunction ButtonPressed))

(event EventAttachPickupAble
  (params (Attach :type Boolean))
  (|CallParentFunction Attach))

(fn ConstructionScript)

(fn RotatePrism
  (params (InputValue :type Vector%202D%20Structure))
  (bind _returnvalue (Utilities|Time|GetWorldDeltaSeconds))
  (bind _returnvalue_2 (* _returnvalue 6e+01))
  (LocalVariables|SetL_xInput (* (.x InputValue) _returnvalue_2))
  (LocalVariables|SetL_yInput (* (.y InputValue) _returnvalue_2))
  (LocalVariables|SetL_NewPrismRotation (Math|Rotator|MakeRotator 0.0 (Math|Float|Clamp(Float) (+ (.pitch (Variables|/Script/Engine.SceneComponent|GetRelativeRotation (Variables|Default|GetBP_RefractingPrism))) (* (LocalVariables|GetL_yInput) (Variables|Default|GetPrismRotationMagnitude))) -15.0 15.0) (+ (* (LocalVariables|GetL_xInput) (Variables|Default|GetPrismRotationMagnitude)) (.yaw (Variables|/Script/Engine.SceneComponent|GetRelativeRotation (Variables|Default|GetBP_RefractingPrism))))))
  (Transformation|SetRelativeRotation (Variables|Default|GetBP_RefractingPrism) (LocalVariables|GetL_NewPrismRotation) false false)
  (bind _asbp_refracting_prism (Utilities|Casting|CastToBP_RefractingPrism (Variables|/Script/Engine.ChildActorComponent|GetChildActor (Variables|Default|GetBP_RefractingPrism))))
  (Default|SetLightBeamDestination _asbp_refracting_prism))