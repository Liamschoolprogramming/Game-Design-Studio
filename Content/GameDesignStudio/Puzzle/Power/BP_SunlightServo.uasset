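; BP_SunlightServo is a puzzle light emitter that casts a beam along its forward vector to power receivers and refracting prisms.
; After a short BeginPlay delay, a looping timer runs EmitLight, a visibility line trace with debug drawing.
; A hit puzzle receiver gets a green signal, while a hit prism refracts the light onward.
; It tracks the lit actor and stops a tracked prism when the beam moves off it.
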(event EventBeginPlay
  (Utilities|FlowControl|Delay 0.5)
  (bind _outactors (Actor|GetAllActorsOfClass "/Game/GameDesignStudio/Possessables/BP_Golem.BP_Golem_C"))
  (bind _output_get (Variables|Default|SetIgnoreActors _outactors))
  (Utilities|Array|Add _output_get (Game|Player|GetPlayerPawn 0))
  (bind _returnvalue (Utilities|Time|SetTimerbyFunctionName 0 "EmitLight" 0.05 true))
  (Variables|Default|SetEmitLightTimer _returnvalue))

(fn ConstructionScript)

(fn EmitLight
  (bind _returnvalue (Transformation|GetActorLocation))
  (bind (_outhit _returnvalue_2) (Collision|LineTraceByChannel _returnvalue (+ _returnvalue (* (Transformation|GetActorForwardVector) (Variables|Default|GetRange))) "TraceTypeQuery1" false 0 "ForDuration"))
  (LocalVariables|SetL_HitActor (.HitActor (Collision|BreakHitResult _outhit)))
  (if _returnvalue_2
    (Utilities|IsValid (Variables|Default|GetReceivingLightActor)
      (:Is%20Valid
        (if (!= (Variables|Default|GetReceivingLightActor) (LocalVariables|GetL_HitActor))
          (bind _asbp_refracting_prism (Utilities|Casting|CastToBP_RefractingPrism (Variables|Default|GetReceivingLightActor) :!label _label))
          (Default|StopLight _asbp_refracting_prism)
          (Variables|Default|SetReceivingLightActor 0)))
      (:Is%20Not%20Valid
        (CallFunction|OnLightReceiverHit (LocalVariables|GetL_HitActor))))
    (else
      (goto _label))))

(fn OnLightReceiverHit
  (params (HitActor :type Actor%20Object%20Reference))
  (bind _aspuzzle_receiver (Utilities|Casting|CastToPuzzleReceiver HitActor)
    (:then
      (LocalVariables|SetL_PuzzleReceiver _aspuzzle_receiver)
      (Variables|Default|SetReceivingLightActor HitActor)
      (Class|PuzzleReceiver|ReceiveGreenSignal (LocalVariables|GetL_PuzzleReceiver) (Variables|Default|GetPuzzleActorGuid)))
    (:CastFailed
      (bind _asbp_refracting_prism (Utilities|Casting|CastToBP_RefractingPrism HitActor)
        (:then
          (Variables|Default|SetReceivingLightActor _asbp_refracting_prism)
          (Default|RefractLight _asbp_refracting_prism self))
        (:CastFailed
          (bind _asbp_refracting_prism_2 (Utilities|Casting|CastToBP_RefractingPrism (Variables|Default|GetReceivingLightActor)))
          (Default|StopLight _asbp_refracting_prism_2))))))