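; BP_SunlightAltar is a puzzle actor that emits a light beam along its forward vector to power puzzle receivers or feed refracting prisms.
; A looping timer, started shortly after BeginPlay, line traces from its point light out to a set range.
; Hits send a green signal to PuzzleReceiver actors or call RefractLight on prisms.
; The Niagara beam's end parameter snaps to the hit target or resets to full range.
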(event EventBeginPlay
  (CallFunction|SetLightBeamEndtoDefault)
  (Utilities|FlowControl|Delay 0.3)
  (bind _outactors (Actor|GetAllActorsOfClass "/Game/GameDesignStudio/Possessables/BP_Golem.BP_Golem_C"))
  (bind _output_get (Variables|Default|SetIgnoreActors _outactors))
  (Utilities|Array|Add _output_get (Game|Player|GetPlayerPawn 0))
  (bind _returnvalue (Utilities|Time|SetTimerbyFunctionName 0 "EmitLight" 0.05 true))
  (Variables|Default|SetEmitLightTimer _returnvalue))

(fn ConstructionScript)

(fn EmitLight
  (bind _pointlight (Variables|Default|GetPointLight))
  (bind _returnvalue (Transformation|GetWorldLocation _pointlight))
  (bind (_outhit _returnvalue_2) (Collision|LineTraceByChannel _returnvalue (+ _returnvalue (* (Transformation|GetActorForwardVector) (Variables|Default|GetRange))) "TraceTypeQuery1" false 0 "ForDuration"))
  (Utilities|IsValid (.HitActor (Collision|BreakHitResult _outhit))
    (:Is%20Valid
      (LocalVariables|SetL_HitActor (.HitActor (Collision|BreakHitResult _outhit))))
    (:Is%20Not%20Valid
      (CallFunction|SetLightBeamEndtoDefault)))
  (if _returnvalue_2
    (Utilities|IsValid (Variables|Default|GetReceivingLightActor)
      (:Is%20Valid
        (if (!= (Variables|Default|GetReceivingLightActor) (LocalVariables|GetL_HitActor))
          (bind _asbp_refracting_prism (Utilities|Casting|CastToBP_RefractingPrism (Variables|Default|GetReceivingLightActor) :!label _label))
          (Default|StopLight _asbp_refracting_prism)
          (Variables|Default|SetReceivingLightActor 0)
          (CallFunction|SetLightBeamEndtoDefault)))
      (:Is%20Not%20Valid
        (CallFunction|OnLightReceiverHit (LocalVariables|GetL_HitActor))
        (goto _label)))))

(fn OnLightReceiverHit
  (params (HitActor :type Actor%20Object%20Reference))
  (bind _aspuzzle_receiver (Utilities|Casting|CastToPuzzleReceiver HitActor)
    (:then
      (LocalVariables|SetL_PuzzleReceiver _aspuzzle_receiver)
      (Variables|Default|SetReceivingLightActor HitActor)
      (Class|PuzzleReceiver|ReceiveGreenSignal (LocalVariables|GetL_PuzzleReceiver) (Variables|Default|GetPuzzleActorGuid))
      (Class|NiagaraComponent|SetNiagaraVariableVec3 (Variables|Default|GetLightBeam) "BeamEnd" (Transformation|GetActorLocation HitActor)))
    (:CastFailed
      (bind _asbp_refracting_prism (Utilities|Casting|CastToBP_RefractingPrism HitActor))
      (Variables|Default|SetReceivingLightActor 0)
      (Default|RefractLight _asbp_refracting_prism self)
      (Class|NiagaraComponent|SetNiagaraVariableVec3 (Variables|Default|GetLightBeam) "BeamEnd" (Transformation|GetWorldLocation (Variables|/Game/GameDesignStudio/Puzzle/Power/BP_RefractingPrism.BP_RefractingPrism_C|GetArrow _asbp_refracting_prism))))))

(fn SetLightBeamEndtoDefault
  (Class|NiagaraComponent|SetNiagaraVariableVec3 (Variables|Default|GetLightBeam) "BeamEnd" (+ (Transformation|GetWorldLocation (Variables|Default|GetPointLight)) (* (Transformation|GetActorForwardVector) (Variables|Default|GetRange)))))