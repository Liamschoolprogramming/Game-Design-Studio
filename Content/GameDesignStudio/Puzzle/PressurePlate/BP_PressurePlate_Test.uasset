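; BP_PressurePlate_Test is a test pressure plate actor for the river puzzle that sinks when a pawn steps on it.
; Sphere overlap swaps the cylinder material between green and red and plays or reverses the Press timeline.
; Timeline updates lower the whole actor from its starting height by PressDepth.
; They also set PressurePlatePressed on the GameManagerSubsystem's puzzle river manager, true only near full depth.
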(event OnComponentBeginOverlap(Sphere)
  (params (OverlappedComponent :type Primitive%20Component%20Object%20Reference) (OtherActor :type Actor%20Object%20Reference) (OtherComp :type Primitive%20Component%20Object%20Reference) (OtherBodyIndex :type Integer) (bFromSweep :type Boolean) (SweepResult :type Hit%20Result%20Structure%20%28by%20ref%29))
  (bind _returnvalue (Transformation|GetActorLocation))
  (bind _returnvalue_2 (Subsystems|GetGameManagerSubsystem))
  (bind _returnvalue_3 (Class|GameManagerSubsystem|GetPuzzleRiverManager _returnvalue_2))
  (if (Class|GameplayStatics|ObjectIsA OtherActor "/Script/Engine.Pawn")
    (CallFunction|Activate)
    (bind _pressdown (Timeline|Press Play)
      (:Update
        (Transformation|SetActorLocation (Math|Vector|MakeVector (.x _returnvalue) (.y _returnvalue) (- (Variables|Default|GetDefaultZPosition) (* _pressdown (Variables|Default|GetPressDepth)))) false false)
        (if (<= (.z (Transformation|GetActorLocation)) (+ (- (Variables|Default|GetDefaultZPosition) (Variables|Default|GetPressDepth)) 0.1))
          (Variables|/Script/GameDesignStudio.PuzzleRiverManager|SetPressurePlatePressed _returnvalue_3 true)
          (else
            (Variables|/Script/GameDesignStudio.PuzzleRiverManager|SetPressurePlatePressed _returnvalue_3 false)))))))

(event OnComponentEndOverlap(Sphere)
  (params (OverlappedComponent :type Primitive%20Component%20Object%20Reference) (OtherActor :type Actor%20Object%20Reference) (OtherComp :type Primitive%20Component%20Object%20Reference) (OtherBodyIndex :type Integer))
  (bind _returnvalue (Transformation|GetActorLocation))
  (bind _returnvalue_2 (Subsystems|GetGameManagerSubsystem))
  (bind _returnvalue_3 (Class|GameManagerSubsystem|GetPuzzleRiverManager _returnvalue_2))
  (CallFunction|Deactivate)
  (bind _pressdown (Timeline|Press Reverse)
    (:Update
      (Transformation|SetActorLocation (Math|Vector|MakeVector (.x _returnvalue) (.y _returnvalue) (- (Variables|Default|GetDefaultZPosition) (* _pressdown (Variables|Default|GetPressDepth)))) false false)
      (if (<= (.z (Transformation|GetActorLocation)) (+ (- (Variables|Default|GetDefaultZPosition) (Variables|Default|GetPressDepth)) 0.1))
        (Variables|/Script/GameDesignStudio.PuzzleRiverManager|SetPressurePlatePressed _returnvalue_3 true)
        (else
          (Variables|/Script/GameDesignStudio.PuzzleRiverManager|SetPressurePlatePressed _returnvalue_3 false))))))

(event EventBeginPlay
  (Variables|Default|SetDefaultZPosition (.z (Transformation|GetActorLocation))))

(fn ConstructionScript)

(fn Activate
  (Rendering|Material|SetMaterial (Variables|Default|GetCylinder) 0 "/Niagara/DefaultAssets/GeometryCache/M_DefaultGeometryCacheMaterial_Green.M_DefaultGeometryCacheMaterial_Green"))

(fn Deactivate
  (Rendering|Material|SetMaterial (Variables|Default|GetCylinder) 0 "/Niagara/DefaultAssets/GeometryCache/M_DefaultGeometryCacheMaterial_Red.M_DefaultGeometryCacheMaterial_Red"))