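; BP_Chest is an interactable puzzle chest that grants its configured rewards to the player once.
; On interact, if its puzzle status is still Start, it marks itself Solved and swaps the chest mesh to a green material as placeholder feedback.
; It shows a WBP_ChestPopup built from the Rewards map, then adds each item and amount to the inventory manager obtained through GameManagerSubsystem.
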(event EventOnInteract
  (params (PlayerCharacter :type Player%20Character%20Object%20Reference))
  (if (Utilities|Enum|Equal(Enum) (Variables|Default|GetPuzzleStatus) "Start")
    (Variables|Default|SetPuzzleStatus "Solved")
    ;[0.15 0.15 0.15 0.5] Play Animations/VFX here
    (Rendering|Material|SetMaterial (Variables|Default|GetChest) 0 "/Game/GameDesignStudio/MaterialLibrary/Debug/M_Green.M_Green")
    ;[0.15 0.15 0.15 0.5] Reward Popup
    (bind _returnvalue (UserInterface|CreateWidget "/Game/GameDesignStudio/UI/ChestPopup/WBP_ChestPopup.WBP_ChestPopup_C" 0 (Variables|Config|GetRewards)))
    (UserInterface|Viewport|AddtoViewport _returnvalue 0)
    ;[0.15 0.15 0.15 0.5] Give Rewards
    (bind (_keypin _valuepin) (Utilities|Map|ForEachLoop(Map) (Variables|Config|GetRewards))
      (:then
        (Class|InventoryManager|AddtoInventory (Class|GameManagerSubsystem|GetInventoryManager (Subsystems|GetGameManagerSubsystem)) _keypin _valuepin)))))

(fn ConstructionScript)