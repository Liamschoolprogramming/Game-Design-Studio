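; BP_RewardPickupable is a puzzle reward pickup that ends the level and grants a stat boost when the player touches it.
; Its Box overlap only reacts to the PlayerCharacter's component tagged PlayerHitBox.
; It then disables all grief objects through the puzzle grief manager, shows and fades in the WBP_LevelEnd widget with game-and-UI input, and calls PickupStatBoost.
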(event OnComponentBeginOverlap(Box)
  (params (OverlappedComponent :type Primitive%20Component%20Object%20Reference) (OtherActor :type Actor%20Object%20Reference) (OtherComp :type Primitive%20Component%20Object%20Reference) (OtherBodyIndex :type Integer) (bFromSweep :type Boolean) (SweepResult :type Hit%20Result%20Structure%20%28by%20ref%29))
  (Utilities|Casting|CastToPlayerCharacter OtherActor)
  (if (Components|ComponentHasTag OtherComp "PlayerHitBox")
    (Class|PuzzleGriefManager|DisableAllGriefObjects (Class|GameManagerSubsystem|GetPuzzleGriefManager (Subsystems|GetGameManagerSubsystem)))
    (bind _returnvalue (UserInterface|CreateWidget "/Game/GameDesignStudio/UI/WBP_LevelEnd.WBP_LevelEnd_C"))
    (UserInterface|Viewport|AddtoViewport _returnvalue 0)
    (Input|SetInputModeGameandUI (Game|GetPlayerController 0) _returnvalue "DoNotLock" true false)
    (Default|FadeinLevelEnd _returnvalue)
    (Class|PuzzleInteractiveStatBooster|PickupStatBoost)))

(fn ConstructionScript)