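; BP_SignalButton is a puzzle button for the vine blockade that toggles one indexed signal.
; On BeginPlay it finds the BP_VineBlockadeManager, which stores the signal states.
; Player overlap with its box, an actor click or the InvertElement event calls ToggleState.
; ToggleState asks the manager to invert the signal and, if that succeeds, colors the cube green for on or red for off.
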(event OnComponentBeginOverlap(Box)
  (params (OverlappedComponent :type Primitive%20Component%20Object%20Reference) (OtherActor :type Actor%20Object%20Reference) (OtherComp :type Primitive%20Component%20Object%20Reference) (OtherBodyIndex :type Integer) (bFromSweep :type Boolean) (SweepResult :type Hit%20Result%20Structure%20%28by%20ref%29))
  (if (Class|GameplayStatics|ObjectIsA OtherActor "/Game/GameDesignStudio/Characters/BP_PlayerCharacter.BP_PlayerCharacter_C")
    (CallFunction|ToggleState)))

(event EventBeginPlay
  (bind _returnvalue (Actor|GetActorOfClass "/Game/GameDesignStudio/Puzzle/VineBlockade/BP_VineBlockadeManager.BP_VineBlockadeManager_C"))
  (Variables|Default|SetManager _returnvalue))

(event EventInvertElement
  (CallFunction|ToggleState))

(event MouseInput|EventActorOnClicked
  (params (ButtonPressed :type Key%20Structure :default "None"))
  (CallFunction|ToggleState))

(fn ConstructionScript)

(fn ToggleState
  (bind _cube (Variables|Default|GetCube))
  (bind _bsuccess (Default|SetSignalState (Variables|Default|GetManager) (Variables|Default|GetSignalIndex) (not (Default|GetSignalState (Variables|Default|GetManager) (Variables|Default|GetSignalIndex)))))
  (if _bsuccess
    (if (Default|GetSignalState (Variables|Default|GetManager) (Variables|Default|GetSignalIndex))
      ;[0.15 0.15 0.15 0.5] Update Materials
      (Rendering|Material|SetMaterial _cube 0 "/Game/GameDesignStudio/MaterialLibrary/Debug/M_Green.M_Green")
      (else
        (Rendering|Material|SetMaterial _cube 0 "/Game/GameDesignStudio/MaterialLibrary/Debug/M_Red.M_Red")))
    (return)))