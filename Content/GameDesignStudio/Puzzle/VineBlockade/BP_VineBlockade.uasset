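; Puzzle vine wall that opens or closes by toggling collision on its vines and invisible box.
; Opens when all recorded emitter signals are green or a budding turret hits it, closing on red or a timer.
; An Inverted puzzle state swaps those responses, and a manager solve locks it open.
; While red, its damage overlap requires the actor be both player and StaticMeshComponent, so likely never fires.
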(event OnComponentBeginOverlap(DamageCollider)
  (params (OverlappedComponent :type Primitive%20Component%20Object%20Reference) (OtherActor :type Actor%20Object%20Reference) (OtherComp :type Primitive%20Component%20Object%20Reference) (OtherBodyIndex :type Integer) (bFromSweep :type Boolean) (SweepResult :type Hit%20Result%20Structure%20%28by%20ref%29))
  (Variables|Default|GetbIsSolved
    (:then)
    (:else
      (if (not (Variables|Default|GetbGreenSignal))
        (if (and (Class|GameplayStatics|ObjectIsA OtherActor "/Game/GameDesignStudio/Characters/BP_PlayerCharacter.BP_PlayerCharacter_C") (Class|GameplayStatics|ObjectIsA OtherActor "/Script/Engine.StaticMeshComponent"))
          (Game|Damage|ApplyDamage OtherActor 1e+02 0 self "/Script/Engine.DamageType"))))))

(event Custom|AutoDeactivate
  ;[0.15 0.15 0.15 0.5] When recieving a green, signal try to open (play); when recieving a red signal, try to close (reverse); if preserved, don't move or change state
  (Variables|Default|GetbIsSolved
    (:then)
    (:else
      (Variables|Default|SetbGreenSignal false)
      (switch Utilities|FlowControl|Switch|SwitchonEPuzzleElementState (Variables|Default|GetPuzzleElementState)
        (:Default
          (CallFunction|Close)
          (Audio|PlaySoundatLocation "/Game/GameDesignStudio/Audio/SFX/Cues/Root_Vine_Wall_sfx_Cue.Root_Vine_Wall_sfx_Cue" (Transformation|GetActorLocation) "0, 0, 0" 1.0 1.0 0.0 0 "/Game/GameDesignStudio/Audio/SFX/Concurrency/Root_Vine_Wall_sfx_Concurrency.Root_Vine_Wall_sfx_Concurrency" 0 0))
        (:Inverted
          (CallFunction|Open))))))

(event EventChangePuzzleActorState
  (params (EPuzzleState :type EPuzzleElementState%20Enum :default "Default"))
  ;[0.15 0.15 0.15 0.5] When recieving a green, signal try to open (play); when recieving a red signal, try to close (reverse); if preserved, don't move or change state
  (Variables|Default|GetbIsSolved
    (:then)
    (:else
      (bind _output_get (Variables|Default|SetPuzzleElementState EPuzzleState))
      (switch Utilities|FlowControl|Switch|SwitchonEPuzzleElementState _output_get
        (:Default
          (if (Variables|Default|GetbGreenSignal)
            (CallFunction|Open :!label _label)
            (else
              (CallFunction|Close :!label _label_2)
              (Audio|PlaySoundatLocation "/Game/GameDesignStudio/Audio/SFX/Cues/Root_Vine_Wall_sfx_Cue.Root_Vine_Wall_sfx_Cue" (Transformation|GetActorLocation) "0, 0, 0" 1.0 1.0 0.0 0 "/Game/GameDesignStudio/Audio/SFX/Concurrency/Root_Vine_Wall_sfx_Concurrency.Root_Vine_Wall_sfx_Concurrency" 0 0))))
        (:Inverted
          (if (Variables|Default|GetbGreenSignal)
            (goto _label_2)
            (else
              (goto _label))))))))

(event EventSolvedbyManager
  (CallFunction|Solve))

(event EventGreenSignal
  (params (EmitterId :type Guid%20Structure))
  ;[0.15 0.15 0.15 0.5] When recieving a green, signal try to open (play); when recieving a red signal, try to close (reverse); if preserved, don't move or change state
  (Variables|Default|GetbIsSolved
    (:then)
    (:else
      (Utilities|Map|Add (Variables|Default|GetSignals) EmitterId true)
      (if (CallFunction|IsFullGreen)
        (Variables|Default|SetbGreenSignal true)
        (switch Utilities|FlowControl|Switch|SwitchonEPuzzleElementState (Variables|Default|GetPuzzleElementState)
          (:Default
            (CallFunction|Open))
          (:Inverted
            (CallFunction|Close)
            (Audio|PlaySoundatLocation "/Game/GameDesignStudio/Audio/SFX/Cues/Root_Vine_Wall_sfx_Cue.Root_Vine_Wall_sfx_Cue" (Transformation|GetActorLocation) "0, 0, 0" 1.0 1.0 0.0 0 "/Game/GameDesignStudio/Audio/SFX/Concurrency/Root_Vine_Wall_sfx_Concurrency.Root_Vine_Wall_sfx_Concurrency" 0 0)))))))

(event EventShotbyBuddingTurret
  ;[0.15 0.15 0.15 0.5] Actiavte vine blockade when shot by a budding turret, then deactivate after 10 seconds
  (Variables|Default|GetbIsSolved
    (:then)
    (:else
      (Utilities|Time|SetTimerbyFunctionName 0 "AutoDeactivate" (Variables|Default|GetOpenOnTurretHitTime))
      ;[0.15 0.15 0.15 0.5] When recieving a green, signal try to open (play); when recieving a red signal, try to close (reverse); if preserved, don't move or change state
      (Variables|Default|SetbGreenSignal true)
      (switch Utilities|FlowControl|Switch|SwitchonEPuzzleElementState (Variables|Default|GetPuzzleElementState)
        (:Default
          (CallFunction|Open))
        (:Inverted
          (CallFunction|Close)
          (Audio|PlaySoundatLocation "/Game/GameDesignStudio/Audio/SFX/Cues/Root_Vine_Wall_sfx_Cue.Root_Vine_Wall_sfx_Cue" (Transformation|GetActorLocation) "0, 0, 0" 1.0 1.0 0.0 0 "/Game/GameDesignStudio/Audio/SFX/Concurrency/Root_Vine_Wall_sfx_Concurrency.Root_Vine_Wall_sfx_Concurrency" 0 0))))))

(event EventRedSignal
  (params (EmitterId :type Guid%20Structure))
  ;[0.15 0.15 0.15 0.5] When recieving a green, signal try to open (play); when recieving a red signal, try to close (reverse); if preserved, don't move or change state
  (Variables|Default|GetbIsSolved
    (:then)
    (:else
      (Utilities|Map|Add (Variables|Default|GetSignals) EmitterId false)
      (Variables|Default|SetbGreenSignal false)
      (switch Utilities|FlowControl|Switch|SwitchonEPuzzleElementState (Variables|Default|GetPuzzleElementState)
        (:Default
          (CallFunction|Close)
          (Audio|PlaySoundatLocation "/Game/GameDesignStudio/Audio/SFX/Cues/Root_Vine_Wall_sfx_Cue.Root_Vine_Wall_sfx_Cue" (Transformation|GetActorLocation) "0, 0, 0" 1.0 1.0 0.0 0 "/Game/GameDesignStudio/Audio/SFX/Concurrency/Root_Vine_Wall_sfx_Concurrency.Root_Vine_Wall_sfx_Concurrency" 0 0))
        (:Inverted
          (CallFunction|Open))))))

(fn ConstructionScript)

(fn Open
  (Collision|SetCollisionResponsetoAllChannels (Variables|Default|GetInvisible%20Box) "ECR_Ignore")
  (Collision|SetCollisionResponsetoAllChannels (Variables|Default|GetVines) "ECR_Ignore"))

(fn Close
  (Collision|SetCollisionResponsetoAllChannels (Variables|Default|GetInvisible%20Box) "ECR_Block")
  (Collision|SetCollisionResponsetoAllChannels (Variables|Default|GetVines) "ECR_Block"))

(fn IsFullGreen
  (bind _valuepin (Utilities|Map|ForEachLoop(Map) (Variables|Default|GetSignals))
    (:then
      (if (!= _valuepin true)
        (return false)))
    (:CompletedPin
      (return true))))

(fn Solve
  (Variables|Default|SetbIsSolved true)
  (CallFunction|Open)
  (Development|PrintString "Solved"))

(fn CheckPuzzleActorState
  (return (Variables|Default|GetPuzzleElementState)))