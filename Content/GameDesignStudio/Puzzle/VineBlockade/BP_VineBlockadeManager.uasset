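; BP_VineBlockadeManager controls a vine blockade puzzle that opens when all of its signals are on.
; BeginPlay fills the signal array with false entries, and SetSignalState updates them unless the manager is locked.
; When the all-signals-on result differs from the current state, it tells the referenced Blockade to open or close.
; Debug text reports signal changes and locked attempts, and a lock-toggle test sits unconnected.
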(event EventBeginPlay
  ;[0.15 0.15 0.15 0.5] Populate bSignals
  (for _index (range 1 (Variables|Config|GetNumSignals))
    (Utilities|Array|Add (Variables|States|GetbSignals) false)))

(fn ConstructionScript)

(fn SetSignalState
  (params (Signal :type Integer) (bState :type Boolean))
  (if (Variables|States|GetbLocked)
    ;[0.15 0.15 0.15 0.5] Debug Display when Locked
    (Development|PrintText (Utilities|Text|FormatText "Vine Blockade is currently locked.") true true "(R=0.000000,G=0.117273,B=0.178125,A=1.000000)")
    (return false)
    (else
      (Utilities|Array|SetArrayElem (Variables|States|GetbSignals) Signal bState)
      (Development|PrintText (Utilities|Text|FormatText "Set Signal [{Index}] to {State}" Signal bState) true true "(R=0.000000,G=0.658375,B=1.000000,A=1.000000)")
      ;[0.15 0.15 0.15 0.5] If resulting blockade state is different than the current, update the blockade state
      (if (!= (CallFunction|IsGreenSignal) (Variables|States|GetbOpen))
        (CallFunction|SetBlockadeState (CallFunction|IsGreenSignal))
        (return true)
        (else
          (return true))))))

(fn IsBlockadeOpen
  (return (Variables|States|GetbOpen)))

(fn IsGreenSignal
  (for _array_element (Variables|States|GetbSignals)
    (if (not _array_element)
      (return false)))
  (return true))

(fn GetSignalState
  (params (Index :type Integer))
  (return (Utilities|Array|Get(acopy) (Variables|States|GetbSignals) Index)))

(fn SetBlockadeState
  (params (bState :type Boolean))
  (bind _output_get (Variables|States|SetbOpen bState))
  (if _output_get
    (Default|Open (Variables|Config|GetBlockade))
    (else
      (Default|Close (Variables|Config|GetBlockade))))
  (return))