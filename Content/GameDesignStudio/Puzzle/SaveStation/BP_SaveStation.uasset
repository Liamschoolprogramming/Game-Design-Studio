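; BP_SaveStation is an interactable save station that registers itself as the save station manager's ActiveSaveStation when used.
; While inactive, a looping timer polls player distance to toggle a billboard prompt and indicator FX within a multiple of InteractRange.
; Interacting or ActivatefromSave sets PuzzleStatus to Active, stopping the poll and hiding both cues.
; Deactivate returns it to Inactive and restarts the loop.
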(event EventActivatefromSave
  (if (Utilities|Enum|NotEqual(Enum) (Variables|Default|GetPuzzleStatus) "Active")
    (CallFunction|Activate)))

(event EventBeginPlay
  (CallFunction|RunCheckforRangeLoop true))

(event EventOnInteract
  (params (PlayerCharacter :type Player%20Character%20Object%20Reference))
  (Development|PrintString "Interacted")
  (Variables|/Script/GameDesignStudio.SaveStationManager|SetActiveSaveStation (Class|GameManagerSubsystem|GetSaveStationManager (Subsystems|GetGameManagerSubsystem)) self)
  (Development|PrintString "Saved")
  (if (Utilities|Enum|NotEqual(Enum) (Variables|Default|GetPuzzleStatus) "Active")
    (CallFunction|Activate)))

(fn ConstructionScript)

(fn Activate
  (Variables|Default|SetPuzzleStatus "Active")
  (CallFunction|RunCheckforRangeLoop false))

(fn Deactivate
  (Variables|Default|SetPuzzleStatus "Inactive")
  (CallFunction|RunCheckforRangeLoop true))

(fn CheckWithinPickupRange
  ;[0.15 0.15 0.15 0.5] If the player is in the interact range, show FX and Press E prompt; Otherwise, disable the FX and don't show the prompt
  (if (<= (Transformation|GetDistanceTo (Game|Player|GetPlayerPawn 0)) (* (Variables|Default|GetInteractRange) 5.0))
    (Rendering|SetVisibility (Variables|Default|GetBillboard) true false)
    (if (not (Components|Activation|IsActive (Variables|Default|GetPickupIndicatorFX)))
      (Components|Activation|Activate (Variables|Default|GetPickupIndicatorFX) false))
    (else
      (Rendering|SetVisibility (Variables|Default|GetBillboard) false false)
      (if (Components|Activation|IsActive (Variables|Default|GetPickupIndicatorFX))
        (Components|Activation|Deactivate (Variables|Default|GetPickupIndicatorFX))))))

(fn RunCheckforRangeLoop
  (params (bRunLoop :type Boolean))
  (if bRunLoop
    (if (not (Utilities|Time|IsTimerActivebyHandle (Variables|Default|GetPickupRangeTimer)))
      (bind _returnvalue (Utilities|Time|SetTimerbyFunctionName 0 "CheckWithinPickupRange" 0.05 true true))
      (Variables|Default|SetPickupRangeTimer _returnvalue))
    (else
      (Components|Activation|Deactivate (Variables|Default|GetPickupIndicatorFX))
      (Rendering|SetVisibility (Variables|Default|GetBillboard) false false)
      (Utilities|Time|ClearandInvalidateTimerbyHandle (Variables|Default|GetPickupRangeTimer)))))