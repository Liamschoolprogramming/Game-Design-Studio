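; Puzzle flower platform that rises on a green signal and lowers on a red one.
; A Grow timeline offsets the platform's Z from its starting height by up to Height, toggling the puzzle status between Active and Start.
; Each rise takes a random duration, while lowering reverses the timeline at a rate scaled by distance from the bottom, with a minimum shrink time.
; Signals are recorded per emitter, but only the current green state gates transitions.
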(event EventGreenSignal
  (params (EmitterId :type Guid%20Structure))
  (bind _platform (Variables|Default|GetPlatform))
  (bind _returnvalue (Transformation|GetWorldLocation _platform))
  ;[0.15 0.15 0.15 0.5] Raise Platform
  (Utilities|Map|Add (Variables|Default|GetSignals) EmitterId true)
  (if (not (Variables|Default|GetbGreenSignal))
    (Variables|Default|SetbGreenSignal true)
    (Variables|Default|SetPuzzleStatus "Active")
    ;;[0.15 0.15 0.15 0.5] Grow Time
    (Components|Timeline|SetPlayRate (Variables|Default|GetGrow) (/ 1.0 (Math|Random|RandomFloatinRange 2.0 3.0)))
    ;[0.15 0.15 0.15 0.5] Grow/Shrink
    (bind _grow (Timeline|Grow Play)
      (:Update
        (Transformation|SetWorldLocation (Variables|Default|GetPlatform) (Math|Vector|MakeVector (.x _returnvalue) (.y _returnvalue) (+ (Variables|Default|GetDefaultHeight) (* _grow (Variables|Config|GetHeight)))) false false)))))

(event EventRedSignal
  (params (EmitterId :type Guid%20Structure))
  (bind _platform (Variables|Default|GetPlatform))
  (bind _returnvalue (Transformation|GetWorldLocation _platform))
  ;[0.15 0.15 0.15 0.5] Lower Platform
  (Utilities|Map|Add (Variables|Default|GetSignals) EmitterId false)
  (if (Variables|Default|GetbGreenSignal)
    (Variables|Default|SetbGreenSignal false)
    (Variables|Default|SetPuzzleStatus "Start")
    ;;[0.15 0.15 0.15 0.5] Lower Time
    (Components|Timeline|SetPlayRate (Variables|Default|GetGrow) (CallFunction|GetShrinkPlaybackRate))
    ;[0.15 0.15 0.15 0.5] Grow/Shrink
    (bind _grow (Timeline|Grow Reverse)
      (:Update
        (Transformation|SetWorldLocation (Variables|Default|GetPlatform) (Math|Vector|MakeVector (.x _returnvalue) (.y _returnvalue) (+ (Variables|Default|GetDefaultHeight) (* _grow (Variables|Config|GetHeight)))) false false)))))

(event EventBeginPlay
  ;[0.15 0.15 0.15 0.5] Set Default Height
  (Variables|Default|SetDefaultHeight (.z (Transformation|GetWorldLocation (Variables|Default|GetPlatform)))))

(fn ConstructionScript)

(fn GetShrinkPlaybackRate
  (return (Math|Float|Min(Float) (/ 1.0 (Math|Float|Max(Float) (/ (- (.z (Transformation|GetWorldLocation (Variables|Default|GetPlatform))) (Variables|Default|GetDefaultHeight)) (Variables|Config|GetShrinkTimeScalar)) 1.0)) (/ 1.0 (Variables|Config|GetMinShrinkTime)))))