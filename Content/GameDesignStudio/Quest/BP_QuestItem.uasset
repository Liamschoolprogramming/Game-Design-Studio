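; BP_QuestItem is a quest item that the player interacts with by walking into it.
; When a PlayerCharacter begins overlapping its Box, it calls Interact with that character; the Interact logic is not defined in this graph.
; SetQuestItemActive shows or hides the Cube and its children, and switches Cube and Box collision between query-only and none.
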(event OnComponentBeginOverlap(Box)
  (params (OverlappedComponent :type Primitive%20Component%20Object%20Reference) (OtherActor :type Actor%20Object%20Reference) (OtherComp :type Primitive%20Component%20Object%20Reference) (OtherBodyIndex :type Integer) (bFromSweep :type Boolean) (SweepResult :type Hit%20Result%20Structure%20%28by%20ref%29))
  (bind _asplayer_character (Utilities|Casting|CastToPlayerCharacter OtherActor))
  (Class|PuzzleInteractiveQuestItem|Interact self _asplayer_character))

(fn ConstructionScript)

(fn SetQuestItemActive
  (params (Active :type Boolean))
  (Rendering|SetVisibility (Variables|Default|GetCube) Active true)
  (if Active
    (Collision|SetCollisionEnabled (Variables|Default|GetCube) "QueryOnly")
    (Collision|SetCollisionEnabled (Variables|Default|GetBox) "QueryOnly")
    (else
      (Collision|SetCollisionEnabled (Variables|Default|GetCube) "NoCollision")
      (Collision|SetCollisionEnabled (Variables|Default|GetBox) "NoCollision"))))