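; BP_QuestStarter is a trigger that starts and completes the quest identified by its QuestKey when the player reaches it.
; Its sphere overlap filters for components tagged PlayerHitBox, then asks the quest manager from the game manager subsystem for the quest state.
; An inactive quest is activated through ActivateQuestForItem, while an active quest is completed if its completion check passes.
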(event OnComponentBeginOverlap(Sphere)
  (params (OverlappedComponent :type Primitive%20Component%20Object%20Reference) (OtherActor :type Actor%20Object%20Reference) (OtherComp :type Primitive%20Component%20Object%20Reference) (OtherBodyIndex :type Integer) (bFromSweep :type Boolean) (SweepResult :type Hit%20Result%20Structure%20%28by%20ref%29))
  (bind _returnvalue (Subsystems|GetGameManagerSubsystem))
  (bind _returnvalue_2 (Class|GameManagerSubsystem|GetQuestManager _returnvalue))
  (if (Components|ComponentHasTag OtherComp "PlayerHitBox")
    (bind _returnvalue_3 (Class|QuestManager|GetQuestState _returnvalue_2 (Variables|Default|GetQuestKey)))
    (switch Utilities|FlowControl|Switch|SwitchonEQuestState _returnvalue_3
      (:INACTIVE
        (Class|QuestManager|ActivateQuestforItem _returnvalue_2 (Variables|Default|GetQuestKey)))
      (:ACTIVE
        (if (Class|QuestManager|CanCompleteQuest _returnvalue_2 (Variables|Default|GetQuestKey))
          (bind _returnvalue_4 (Class|QuestManager|CompleteQuest (Class|GameManagerSubsystem|GetQuestManager (Subsystems|GetGameManagerSubsystem)) (Variables|Default|GetQuestKey))))))))

(fn ConstructionScript)