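; Possessable crystal beetle that carries a refracting prism the player can rotate.
; Construction runs the parent script, then sets the player character type to Beetle.
; RotatePrism scales 2D input by a rotation magnitude and adds it to the prism's relative rotation, with X driving free yaw, Y driving clamped pitch, and roll held at zero.
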(event EventBeginPlay
  (|CallParentFunction))

(fn ConstructionScript
  (|CallParentFunction)
  (Variables|Default|SetPlayerCharacterType "Beetle"))

(fn RotatePrism
  (params (InputValue :type Vector%202D%20Structure))
  (LocalVariables|SetL_XInput (.x InputValue))
  (LocalVariables|SetL_YInput (.y InputValue))
  (LocalVariables|SetL_NewPrismRotation (Math|Rotator|MakeRotator 0.0 (Math|Float|Clamp(Float) (+ (.pitch (Variables|/Script/Engine.SceneComponent|GetRelativeRotation (Variables|Default|GetBP_RefractingPrism))) (* (LocalVariables|GetL_YInput) (Variables|Default|GetPrismRotationMagnitude))) -15.0 15.0) (+ (* (LocalVariables|GetL_XInput) (Variables|Default|GetPrismRotationMagnitude)) (.yaw (Variables|/Script/Engine.SceneComponent|GetRelativeRotation (Variables|Default|GetBP_RefractingPrism))))))
  (Transformation|SetRelativeRotation (Variables|Default|GetBP_RefractingPrism) (LocalVariables|GetL_NewPrismRotation) false false))