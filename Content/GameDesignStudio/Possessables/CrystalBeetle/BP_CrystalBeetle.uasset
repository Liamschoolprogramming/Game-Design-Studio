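; Possessable crystal beetle that carries a refracting prism the player can rotate to aim a light beam.
; RotatePrism turns input into yaw and clamped pitch on the child actor prism, then tells it to update its beam destination.
; Construction tags it as the Beetle character type.
; On first possession it shows a hint popup from DT_Hints and marks its tutorial completed through the game manager's tutorial manager.
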(event EventBeginPlay
  (|CallParentFunction))

(fn ConstructionScript
  (|CallParentFunction)
  (Variables|Default|SetPlayerCharacterType "Beetle"))

(fn RotatePrism
  (params (InputValue :type Vector%202D%20Structure))
  (LocalVariables|SetL_xInput (.x InputValue))
  (LocalVariables|SetL_yInput (.y InputValue))
  (LocalVariables|SetL_NewPrismRotation (Math|Rotator|MakeRotator 0.0 (Math|Float|Clamp(Float) (+ (.pitch (Variables|/Script/Engine.SceneComponent|GetRelativeRotation (Variables|Default|GetBP_RefractingPrism))) (* (LocalVariables|GetL_yInput) (Variables|Default|GetPrismRotationMagnitude))) -15.0 15.0) (+ (* (LocalVariables|GetL_xInput) (Variables|Default|GetPrismRotationMagnitude)) (.yaw (Variables|/Script/Engine.SceneComponent|GetRelativeRotation (Variables|Default|GetBP_RefractingPrism))))))
  (Transformation|SetRelativeRotation (Variables|Default|GetBP_RefractingPrism) (LocalVariables|GetL_NewPrismRotation) false false)
  (bind _asbp_refracting_prism (Utilities|Casting|CastToBP_RefractingPrism (Variables|/Script/Engine.ChildActorComponent|GetChildActor (Variables|Default|GetBP_RefractingPrism))))
  (Default|SetLightBeamDestination _asbp_refracting_prism))

(fn OnPossessedFinish
  (|CallParentFunction)
  ;[0.15 0.15 0.15 0.5] Prompt Tutorial on First Possess
  (if (Utilities|Enum|Equal(Enum) (Class|TutorialManager|GetCurrentStage (Class|GameManagerSubsystem|GetTutorialManager (Subsystems|GetGameManagerSubsystem)) "CrystalBeetle") "NotStarted")
    (Class|BPIHUD|DisplayPopupNotification(Message) (HUD|GetHUD (Game|GetPlayerController 0)) (Utilities|Struct|MakeDataTableRowHandle "/Game/GameDesignStudio/Tutorial/DT_Hints.DT_Hints" "CrystalBeetle"))
    (Class|TutorialManager|SetTutorialStage (Class|GameManagerSubsystem|GetTutorialManager (Subsystems|GetGameManagerSubsystem)) "CrystalBeetle" "Completed")))