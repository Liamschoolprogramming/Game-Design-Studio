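; Possessable entity Blueprint that shows a Niagara indicator when the player is able to possess it.
; On BeginPlay it caches the HUD and derives possess range from the player's base range plus a Mind Points bonus.
; A looping one-second timer toggles the indicator by eligibility and distance, hiding it on the currently controlled character.
; Possession start recolours the indicator, and finish notifies the HUD and clears the highlight.
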(event Custom|CheckWithinRange
  (bind _asplayer_controller_base (Utilities|Casting|CastToPlayerControllerBase (Game|GetPlayerController 0)))
  (bind _possessableindicatorniagaracomponent (Variables|Default|GetPossessableIndicatorNiagaraComponent)
    (:then
      (bind _returnvalue (Class|PlayerControllerBase|CanPossessEntity _asplayer_controller_base self))
      (if (== (Game|GetPlayerCharacter 0) self)
        (if (Components|Activation|IsActive _possessableindicatorniagaracomponent) :!label _label
          (Components|Activation|Deactivate _possessableindicatorniagaracomponent)
          (Niagara|SetNiagaraVariable(LinearColor) (Variables|Default|GetPossessableIndicatorNiagaraComponent) "Colour" (Variables|Default|GetDefaultColour) :!label _label_2))
        (elif (and _returnvalue (<= (Math|Vector|Distance(Vector) (Transformation|GetActorLocation (Game|GetPlayerCharacter 0)) (Transformation|GetActorLocation)) (Variables|Default|GetPossess%20Range)))
          (if (not (Components|Activation|IsActive _possessableindicatorniagaracomponent))
            (Components|Activation|Activate _possessableindicatorniagaracomponent true)
            (goto _label_2))
          (else
            (goto _label)))))
    (:else)))

(event EventBeginPlay
  (bind _asbp_hud (Utilities|Casting|CastToBP_HUD (HUD|GetHUD (Game|GetPlayerController 0))))
  (Variables|Default|SetHUD _asbp_hud)
  (bind _returnvalue (Class|PlayerStatManager|GetPlayerStats (Class|GameManagerSubsystem|GetPlayerStatManager (Subsystems|GetGameManagerSubsystem))))
  ;[0.15 0.15 0.15 0.5 14] multiply mind points +  default possess range for basic interaction
  (Variables|Default|SetPossess%20Range (+ (.PossessRange (Utilities|Struct|BreakPlayerStats _returnvalue)) (* (.MindPoints (Utilities|Struct|BreakPlayerStats _returnvalue)) 5.0)))
  (Utilities|Time|SetTimerbyEvent (delegate Custom|CheckWithinRange) 1.0 true true))

(fn ConstructionScript)

(fn OnPossessedStart
  (Niagara|SetNiagaraVariable(LinearColor) (Variables|Default|GetPossessableIndicatorNiagaraComponent) "Colour" (Variables|Default|GetConfirmColour)))

(fn OnPossessedFinish
  (Default|OnConfirmPossession (Variables|Default|GetHUD))
  (CallFunction|OnSetHighlight false))