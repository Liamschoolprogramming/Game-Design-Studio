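; Possessable budding flower turret that the player rotates left and right to shoot projectiles.
; Holding the jump input, a temporary fire binding, plays a bloom montage, then starts a looping timer spawning short-lived projectiles until release.
; A separate cooldown timer gates restarting fire.
; Possession locks camera rotation and zoom, shows a crosshair and triggers a one-time tutorial hint; unpossession restores the camera and removes the crosshair.
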(event Custom|Reset%20CanManuallyFire
  ;[0.15 0.15 0.15 0.5] (Using jump IA temporarily) Started projectile for loop when holding the fire button and breaks the loop if the button is released
  (Variables|Default|SetbCanFire? true))

(event Input|EnhancedActionEvents|EnhancedInputActionIA_Move
  (params (ActionValue :type Vector%202D%20Structure) (ElapsedSeconds :type Float%20%28double-precision%29) (TriggeredSeconds :type Float%20%28double-precision%29) (InputAction :type Input%20Action%20Object%20Reference :default "/Game/GameDesignStudio/Input/Actions/IA_Move.IA_Move"))
  ;[0.15 0.15 0.15 0.5] Rotates head based on left/right move input
  (CallFunction|Aim (.x ActionValue)))

(event Input|EnhancedActionEvents|EnhancedInputActionIA_Jump
  (params (ActionValue :type Boolean) (ElapsedSeconds :type Float%20%28double-precision%29) (TriggeredSeconds :type Float%20%28double-precision%29) (InputAction :type Input%20Action%20Object%20Reference :default "/Game/GameDesignStudio/Input/Actions/IA_Jump.IA_Jump"))
  ;[0.15 0.15 0.15 0.5] (Using jump IA temporarily) Started projectile for loop when holding the fire button and breaks the loop if the button is released
  (:Started
    (Variables|Default|SetbWantsToFire true)
    (if (Variables|Default|GetbCanFire?)
      (Variables|Default|SetbCanFire? false)
      (Animation|Montage|PlayMontage (Variables|Character|GetMesh) "/Game/GameDesignStudio/Art/BloomingFlowerTurret/AM_Blooming_Flower_Transition.AM_Blooming_Flower_Transition"
        (:OnCompleted
          (CallFunction|FireBuddingTurret)
          (Audio|PlaySoundatLocation "/Game/GameDesignStudio/Audio/SFX/Cues/Pellet_shot_sfx_Cue.Pellet_shot_sfx_Cue" (Transformation|GetActorLocation) "0, 0, 0" 1.0 1.0 0.0 0 "/Game/GameDesignStudio/Audio/SFX/Concurrency/Pellet_shot_sfx_Concurrency.Pellet_shot_sfx_Concurrency" 0 0)
          (bind _returnvalue (Utilities|Time|SetTimerbyEvent (delegate Custom|Reset%20CanManuallyFire) (+ (Variables|Default|GetFireRate) 1.0)))
          (Variables|Default|SetFireCooldownTimer _returnvalue))
        (:OnInterrupted
          (Variables|Default|SetbCanFire? true)))))
  (:Canceled
    (Variables|Default|SetbWantsToFire false :!label _label)
    (Utilities|Time|ClearandInvalidateTimerbyHandle (Variables|Default|GetFiringTimer)))
  (:Completed
    (goto _label)))

(event EventBeginPlay
  ;[0.15 0.15 0.15 0.5] Create crosshair WBP
  (|CallParentFunction)
  (bind _returnvalue (UserInterface|CreateWidget "/Game/GameDesignStudio/UI/TurretCrosshair/WBP_TurretCrosshair.WBP_TurretCrosshair_C"))
  (Variables|Default|SetWBP_Crosshair _returnvalue))

(event EventUnpossessed
  (params (OldController :type Controller%20Object%20Reference))
  ;[0.15 0.15 0.15 0.5] Hides crosshair widget
  (|CallParentFunction OldController)
  (Utilities|IsValid (Game|Player|GetPlayerPawn 0)
    (:Is%20Valid
      (Widget|RemovefromParent (Variables|Default|GetWBP_Crosshair))
      ;[0.15 0.15 0.15 0.5] Disables independent camera movement on possession
      (bind _bp_player_controller (Class|BPIPlayerControllerPossession|GetBPPlayerController(Message) (Game|GetPlayerController 0)))
      (Variables|/Script/GameDesignStudio.CustomCamera|SetbLetCameraRotate (Variables|/Script/GameDesignStudio.PlayerControllerBase|GetCameraReference _bp_player_controller) true)
      (Variables|/Script/GameDesignStudio.CustomCamera|SetbLetCameraZoom (Variables|/Script/GameDesignStudio.PlayerControllerBase|GetCameraReference _bp_player_controller) true))))

(fn ConstructionScript
  (|CallParentFunction)
  (Variables|Default|SetPlayerCharacterType "Turret"))

(fn Aim
  (params (Yaw :type Float%20%28double-precision%29))
  (bind _returnvalue (Transformation|GetActorRotation))
  ;[0.15 0.15 0.15 0.5] Rotates only left right movement input
  (Pawn|Input|AddControllerYawInput (* Yaw (* (Utilities|Time|GetWorldDeltaSeconds) 6e+01)))
  (Transformation|SetActorRotation (Math|Rotator|MakeRotator (.roll _returnvalue) (.pitch _returnvalue) (.yaw (Pawn|GetControlRotation :!class /Script/Engine.Pawn)))))

(fn FireBuddingTurret
  ;[0.15 0.15 0.15 0.5] Firing (Sets loop to automatically fire as long as button is held)
  (if (not (Utilities|Time|IsTimerActivebyHandle (Variables|Default|GetFiringTimer)))
    (bind _returnvalue (Utilities|Time|SetTimerbyFunctionName 0 "FiringLoop" (Variables|Default|GetFireRate) true false (* (Variables|Default|GetFireRate) -1.0)))
    (Variables|Default|SetFiringTimer _returnvalue)))

(fn FiringLoop
  (bind _mesh (Variables|Character|GetMesh))
  (bind _returnvalue (Transformation|GetWorldLocation _mesh))
  ;[0.15 0.15 0.15 0.5] Fires projectiles from the barrel
  (if (Variables|Default|GetbWantsToFire)
    (Collision|LineTraceByChannel _returnvalue (+ _returnvalue (* (Math|Vector|GetRightVector (Variables|Character|GetMesh)) 4e+03)) "TraceTypeQuery1" false 0 "ForDuration" true "(R=1.000000,G=0.000000,B=0.000000,A=1.000000)" "(R=0.000000,G=1.000000,B=0.000000,A=1.000000)" 0.7)
    (CallFunction|SpawnProjectile)
    (else
      (Utilities|Time|ClearandInvalidateTimerbyHandle (Variables|Default|GetFiringTimer)))))

(fn SpawnProjectile
  ;[0.15 0.15 0.15 0.5] Spawns projectiles from barrel location and sets limited lifespan
  (bind _returnvalue (Game|SpawnActorfromClass "/Game/GameDesignStudio/Projectiles/BP_ProjectileBuddingTurret.BP_ProjectileBuddingTurret_C" (Math|Transform|MakeTransform (Transformation|GetWorldLocation (Variables|Default|GetAimArrow)) (Transformation|GetWorldRotation (Variables|Default|GetAimArrow)) "1.000000,1.000000,1.000000") "Undefined" "MultiplyWithRoot" 0 0))
  (Actor|SetLifeSpan _returnvalue 2.0))

(fn OnPossessedFinish
  (|CallParentFunction)
  ;[0.15 0.15 0.15 0.5] Disables independent camera movement on possession
  (bind _bp_player_controller (Class|BPIPlayerControllerPossession|GetBPPlayerController(Message) (Game|GetPlayerController 0)))
  (Variables|/Script/GameDesignStudio.CustomCamera|SetbLetCameraRotate (Variables|/Script/GameDesignStudio.PlayerControllerBase|GetCameraReference _bp_player_controller) false)
  (Variables|/Script/GameDesignStudio.CustomCamera|SetbLetCameraZoom (Variables|/Script/GameDesignStudio.PlayerControllerBase|GetCameraReference _bp_player_controller) false)
  ;[0.15 0.15 0.15 0.5] Shows crosshair widget
  (UserInterface|Viewport|AddtoViewport (Variables|Default|GetWBP_Crosshair) 0)
  ;[0.15 0.15 0.15 0.5] Prompt Tutorial on First Possess
  (if (Utilities|Enum|Equal(Enum) (Class|TutorialManager|GetCurrentStage (Class|GameManagerSubsystem|GetTutorialManager (Subsystems|GetGameManagerSubsystem)) "BuddingTurret") "NotStarted")
    (Class|BPIHUD|DisplayPopupNotification(Message) (HUD|GetHUD (Game|GetPlayerController 0)) (Utilities|Struct|MakeDataTableRowHandle "/Game/GameDesignStudio/Tutorial/DT_Hints.DT_Hints" "BuddingTurret"))
    (Class|TutorialManager|SetTutorialStage (Class|GameManagerSubsystem|GetTutorialManager (Subsystems|GetGameManagerSubsystem)) "BuddingTurret" "Completed")))