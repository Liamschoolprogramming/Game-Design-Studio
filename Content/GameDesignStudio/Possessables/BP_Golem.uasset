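; BP_Golem is a possessable Golem pawn, built on a shared possessable parent and typed as Golem in its construction script.
; Possession swaps the mesh to an active material, lowers the player controller's movement speed and overrides the camera zoom.
; Input stays disabled during the possession montage and returns when it completes or is interrupted.
; Unpossessing restores the inactive material and the faster movement speed.
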(event EventBeginPlay
  (|CallParentFunction)
  (Rendering|Material|SetMaterial (Variables|Character|GetMesh) 0 "/Game/GameDesignStudio/Characters/Golem/Golem_updated/MI_Inactive.MI_Inactive"))

(event EventPossessed
  (params (NewController :type Controller%20Object%20Reference))
  (bind _returnvalue (Game|GetPlayerController 0))
  (bind _returnvalue_2 (Game|GetPlayerController 0))
  (|CallParentFunction NewController)
  (Rendering|Material|SetMaterial (Variables|Character|GetMesh) 0 "/Game/GameDesignStudio/Characters/Golem/Golem_updated/MI_Active.MI_Active")
  (Utilities|IsValid _returnvalue
    (:Is%20Valid
      (Input|DisableInput _returnvalue _returnvalue)
      (bind _asbp_player_controller (Utilities|Casting|CastToBP_PlayerController _returnvalue))
      (Variables|/Script/GameDesignStudio.PlayerControllerBase|SetPawnMovementSpeed _asbp_player_controller 4e+02)
      (bind _camerareference (Variables|/Script/GameDesignStudio.PlayerControllerBase|GetCameraReference _asbp_player_controller)
        (:then
          (Class|CustomCamera|OverrideZoom _camerareference 0.75 false)
          (Animation|Montage|PlayMontage (Variables|Character|GetMesh) "/Game/GameDesignStudio/Characters/Golem/AM_Golem_Possesed_New.AM_Golem_Possesed_New"
            (:OnCompleted
              _)
            (:OnInterrupted
              _))
          (Input|EnableInput _returnvalue_2 _returnvalue_2))
        (:else)))))

(event EventUnpossessed
  (params (OldController :type Controller%20Object%20Reference))
  (bind _returnvalue (Game|GetPlayerController 0))
  (|CallParentFunction OldController)
  (Rendering|Material|SetMaterial (Variables|Character|GetMesh) 0 "/Game/GameDesignStudio/Characters/Golem/Golem_updated/MI_Inactive.MI_Inactive")
  (Utilities|IsValid _returnvalue
    (:Is%20Valid
      (bind _asbp_player_controller (Utilities|Casting|CastToBP_PlayerController _returnvalue))
      (Variables|/Script/GameDesignStudio.PlayerControllerBase|SetPawnMovementSpeed _asbp_player_controller 5e+02))))

(fn ConstructionScript
  (|CallParentFunction)
  (Variables|Default|SetPlayerCharacterType "Golem"))