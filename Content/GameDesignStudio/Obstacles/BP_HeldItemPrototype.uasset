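; Prototype pickup item that the player collects to interact with item gates in the level.
; On BeginPlay it finds every BP_ItemGate, adds itself to each gate's HoldableItems and has the gate bind to it.
; When a PlayerCharacter overlaps its sphere, it sets the player's HasItem flag, calls GetItem to signal the pickup and destroys itself.
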(event OnComponentBeginOverlap(Sphere)
  (params (OverlappedComponent :type Primitive%20Component%20Object%20Reference) (OtherActor :type Actor%20Object%20Reference) (OtherComp :type Primitive%20Component%20Object%20Reference) (OtherBodyIndex :type Integer) (bFromSweep :type Boolean) (SweepResult :type Hit%20Result%20Structure%20%28by%20ref%29))
  (bind _asplayer_character (Utilities|Casting|CastToPlayerCharacter OtherActor))
  (Variables|/Script/GameDesignStudio.PlayerCharacter|SethasItem _asplayer_character true)
  (Default|CallGetItem)
  (Actor|DestroyActor))

(event EventBeginPlay
  (bind _self self)
  (bind _outactors (Actor|GetAllActorsOfClass "/Game/GameDesignStudio/Obstacles/BP_ItemGate.BP_ItemGate_C"))
  (for _array_element _outactors
    (Utilities|Array|Add (Variables|/Game/GameDesignStudio/Obstacles/BP_ItemGate.BP_ItemGate_C|GetHoldableItems _array_element) _self)
    (Default|BindItem _array_element _self)))

(fn ConstructionScript)