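; BP_ItemGate is an obstacle that stops the player carrying pickupable puzzle items through it.
; A pickupable entering its box is dropped and swept to an offset along player 0's right vector.
; An overlapping player gets IsInItemGate set, provided the gate's overlapped component carries the PlayerHitBox tag.
; Ending the overlap clears that flag.
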(event OnComponentBeginOverlap(Box)
  (params (OverlappedComponent :type Primitive%20Component%20Object%20Reference) (OtherActor :type Actor%20Object%20Reference) (OtherComp :type Primitive%20Component%20Object%20Reference) (OtherBodyIndex :type Integer) (bFromSweep :type Boolean) (SweepResult :type Hit%20Result%20Structure%20%28by%20ref%29))
  (CallFunction|HandleItemDrop OverlappedComponent OtherActor))

(event OnComponentEndOverlap(Box)
  (params (OverlappedComponent :type Primitive%20Component%20Object%20Reference) (OtherActor :type Actor%20Object%20Reference) (OtherComp :type Primitive%20Component%20Object%20Reference) (OtherBodyIndex :type Integer))
  ;[0.15 0.15 0.15 0.5] Stopped overlapping player, player can get pickupable
  (bind _asplayer_character (Utilities|Casting|CastToPlayerCharacter OtherActor))
  (Variables|/Script/GameDesignStudio.PlayerCharacter|SetbIsInItemGate _asplayer_character false))

(fn ConstructionScript)

(fn HandleItemDrop
  (params (OverlappedComponent :type Primitive%20Component%20Object%20Reference) (OverlappedActor :type Actor%20Object%20Reference))
  (bind _returnvalue (Game|GetPlayerCharacter 0))
  (bind _aspuzzle_interactive_pickupable (Utilities|Casting|CastToPuzzleInteractive_Pickupable OverlappedActor)
    (:then
      (LocalVariables|SetL_Pickupable _aspuzzle_interactive_pickupable)
      ;[0.15 0.15 0.15 0.5] Overlapped Pickupable, Drop to side of player
      (Class|PuzzleInteractivePickupable|Drop (LocalVariables|GetL_Pickupable))
      (Transformation|SetActorTransform (LocalVariables|GetL_Pickupable) (Math|Transform|MakeTransform (+ (Transformation|GetActorLocation _returnvalue) (* (Transformation|GetActorRightVector _returnvalue) "200.000000,200.000000,0.000000")) (Transformation|GetActorRotation (LocalVariables|GetL_Pickupable)) "1.000000,1.000000,1.000000") true true))
    (:CastFailed
      ;[0.15 0.15 0.15 0.5] Overlapped Player, Player cannot get pickupable
      (bind _asplayer_character (Utilities|Casting|CastToPlayerCharacter OverlappedActor))
      (if (Components|ComponentHasTag OverlappedComponent "PlayerHitBox")
        (Variables|/Script/GameDesignStudio.PlayerCharacter|SetbIsInItemGate _asplayer_character true)))))