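; Blooming flower turret obstacle that swivels toward the player and shoots projectiles while they are inside its forward vision box.
; Looping timers, rather than Tick, interpolate the head's yaw toward the target, or back to its starting rotation once the player leaves.
; A firing-loop timer plays the shoot montage and spawns a projectile only when a line trace hits the player.
; A Budding Turret shot disables it for ten seconds.
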(event OnComponentBeginOverlap(VisionBox)
  (params (OverlappedComponent :type Primitive%20Component%20Object%20Reference) (OtherActor :type Actor%20Object%20Reference) (OtherComp :type Primitive%20Component%20Object%20Reference) (OtherBodyIndex :type Integer) (bFromSweep :type Boolean) (SweepResult :type Hit%20Result%20Structure%20%28by%20ref%29))
  ;[0.15 0.15 0.15 0.5] When player setps into vision range, rotate to face player and start shooting
  (if (and (Class|GameplayStatics|ObjectIsA OtherActor "/Game/GameDesignStudio/Characters/BP_PlayerCharacter.BP_PlayerCharacter_C") (not (Class|GameplayStatics|ObjectIsA OtherComp "/Script/Engine.SphereComponent")))
    (Variables|Default|SetTargetRef OtherActor)
    (if (not (Variables|Default|GetbDisabled))
      (if (Variables|Default|GetbCanFire?)
        (Variables|Default|SetbCanFire? false)
        (CallFunction|FireBloomingTurret)
        (Utilities|Time|ClearandInvalidateTimerbyHandle (Variables|Default|GetReturnRotateTimer))
        (bind _returnvalue (Utilities|Time|SetTimerbyFunctionName 0 "RotateToTarget" 0.01 true true))
        (Variables|Default|SetAttackRotateTimer _returnvalue)))))

(event OnComponentEndOverlap(VisionBox)
  (params (OverlappedComponent :type Primitive%20Component%20Object%20Reference) (OtherActor :type Actor%20Object%20Reference) (OtherComp :type Primitive%20Component%20Object%20Reference) (OtherBodyIndex :type Integer))
  ;[0.15 0.15 0.15 0.5] When player exits sight range, stop shooting and return to rest
  (if (Class|GameplayStatics|ObjectIsA OtherActor "/Game/GameDesignStudio/Characters/BP_PlayerCharacter.BP_PlayerCharacter_C")
    (if (not (Variables|Default|GetbDisabled))
      (Utilities|Time|ClearandInvalidateTimerbyHandle (Variables|Default|GetFiringTimer))
      (Utilities|Time|ClearandInvalidateTimerbyHandle (Variables|Default|GetFiringTimer))
      (Variables|Default|SetbCanFire? true)
      (Variables|Default|SetTargetRef 0)
      (CallFunction|ReturntoRest))))

(event Custom|Enable
  ;[0.15 0.15 0.15 0.5] Enables turret movement after 10 second timer ends; If player is still visible, go back to attacking; If player is out of view, go back to rest
  (Variables|Default|SetbDisabled false)
  (if (Collision|IsOverlappingActor (Variables|Default|GetVisionBox) (Variables|Default|GetTargetRef) :!class /Script/Engine.PrimitiveComponent)
    (CallFunction|FireBloomingTurret)
    (else
      (Variables|Default|SetbCanFire? true)
      (Variables|Default|SetTargetRef 0)
      (CallFunction|ReturntoRest))))

(event Custom|FiringMontage
  (Animation|Montage|PlayMontage (Variables|Default|GetSkeletalMesh) "/Game/GameDesignStudio/Art/BloomingFlowerTurret/AM_Flower_Turret_Shoot_New.AM_Flower_Turret_Shoot_New"))

(event EventShotbyBuddingTurret
  ;[0.15 0.15 0.15 0.5] Stops attacking and rotating while disabled by budding turret
  (Variables|Default|SetbDisabled true)
  (Utilities|Time|ClearandInvalidateTimerbyHandle (Variables|Default|GetFiringTimer))
  (Utilities|Time|ClearandInvalidateTimerbyHandle (Variables|Default|GetAttackRotateTimer))
  (Utilities|Time|SetTimerbyEvent (delegate Custom|Enable) 1e+01))

(event EventBeginPlay
  ;[0.15 0.15 0.15 0.5] Sets default rotation (which is also the rotation it will return to when not hostile)
  (Variables|Default|SetDefaultRotation (Transformation|GetActorRotation))
  (Components|Box|SetBoxExtent (Variables|Default|GetVisionBox) (Math|Vector|MakeVector 1.2e+02 (Variables|Default|GetVisionRange) 9e+01) true)
  (Transformation|SetRelativeLocation (Variables|Default|GetVisionBox) (Math|Vector|MakeVector 0.0 (+ (Variables|Default|GetVisionRange) 8.0) 9e+01) false false))

(fn ConstructionScript
  (|CallParentFunction))

(fn Aim
  (params (Yaw :type Float%20%28double-precision%29))
  (bind _skeletalmesh (Variables|Default|GetSkeletalMesh))
  (bind _relativerotation (Variables|/Script/Engine.SceneComponent|GetRelativeRotation _skeletalmesh))
  ;[0.15 0.15 0.15 0.5] Rotates only left right movement input
  (Pawn|Input|AddControllerYawInput Yaw)
  (Transformation|SetRelativeRotation (Variables|Default|GetSkeletalMesh) (Math|Rotator|MakeRotator (.roll _relativerotation) (.pitch _relativerotation) (.yaw (Pawn|GetControlRotation :!class /Script/Engine.Pawn))) false false))

(fn FireBloomingTurret
  ;[0.15 0.15 0.15 0.5] Firing (Sets loop to automatically fire as long as button is held)
  (if (not (Utilities|Time|IsTimerActivebyHandle (Variables|Default|GetFiringTimer)))
    (bind _returnvalue (Utilities|Time|SetTimerbyFunctionName 0 "FiringLoop" (Variables|Default|GetFireRate) true false (* (Variables|Default|GetFireRate) -1.0)))
    (Variables|Default|SetFiringTimer _returnvalue)
    (Variables|Default|SetIsFiring true)))

(fn FiringLoop
  (bind _skeletalmesh (Variables|Default|GetSkeletalMesh))
  (bind _returnvalue (Transformation|GetWorldLocation _skeletalmesh))
  (bind (_x _y _z) (Math|Vector|BreakVector _returnvalue))
  ;[0.15 0.15 0.15 0.5] Fires projectile only if player is hit by the line trace (ie in front of the barrel)
  (bind _outhit (Collision|LineTraceByChannel (Math|Vector|MakeVector _x _y (+ _z 1e+02)) (+ _returnvalue (* (Math|Vector|GetRightVector (Variables|Default|GetSkeletalMesh)) 4e+03)) "TraceTypeQuery2" false (Utilities|Array|MakeArray self) "None" true "(R=1.000000,G=0.000000,B=0.000000,A=1.000000)" "(R=0.000000,G=1.000000,B=0.000000,A=1.000000)" 0.7))
  (if (Class|GameplayStatics|ObjectIsA (.HitActor (Collision|BreakHitResult _outhit)) "/Game/GameDesignStudio/Characters/BP_PlayerCharacter.BP_PlayerCharacter_C")
    (CallFunction|FiringMontage)
    (CallFunction|SpawnProjectile)))

(fn SpawnProjectile
  (bind _skeletalmesh (Variables|Default|GetSkeletalMesh))
  (bind _returnvalue (Transformation|GetSocketLocation _skeletalmesh "FiringSocket"))
  ;[0.15 0.15 0.15 0.5] Spawns projectile actor from barrel
  (bind _returnvalue_2 (Game|SpawnActorfromClass "/Game/GameDesignStudio/Projectiles/BP_ProjectileBloomingTurret.BP_ProjectileBloomingTurret_C" (Math|Transform|MakeTransform _returnvalue (Math|Rotator|FindLookatRotation _returnvalue (Transformation|GetActorLocation (Variables|Default|GetTargetRef))) "1.000000,1.000000,1.000000") "Undefined" "MultiplyWithRoot" 0 0))
  (Actor|SetLifeSpan _returnvalue_2 2.0))

(fn ReturntoRest
  ;[0.15 0.15 0.15 0.5] Calls Loop To Return to Rest After Losing the Target
  (Utilities|Time|ClearandInvalidateTimerbyHandle (Variables|Default|GetAttackRotateTimer))
  (bind _returnvalue (Utilities|Time|SetTimerbyFunctionName 0 "GoBack" 0.01 true true))
  (Variables|Default|SetReturnRotateTimer _returnvalue)
  (Variables|Default|SetIsFiring false))

(fn GoBack
  (bind _defaultrotation (Variables|Default|GetDefaultRotation))
  ;[0.15 0.15 0.15 0.5] Loop that rotates head back to default rotation
  (Transformation|SetWorldRotation (Variables|Default|GetSkeletalMesh) (Math|Rotator|MakeRotator (.roll _defaultrotation) (.pitch _defaultrotation) (.yaw (Math|Interpolation|RInterpTo (Transformation|GetWorldRotation (Variables|Default|GetSkeletalMesh)) (Variables|Default|GetDefaultRotation) 1.0 0.025))) false false)
  (if (== (Math|Float|Round (.yaw (Transformation|GetWorldRotation (Variables|Default|GetSkeletalMesh)))) (Math|Float|Round (.yaw (Variables|Default|GetDefaultRotation))))
    (Utilities|Time|ClearandInvalidateTimerbyHandle (Variables|Default|GetReturnRotateTimer))))

(fn RotatetoTarget
  (bind _defaultrotation (Variables|Default|GetDefaultRotation))
  (bind _skeletalmesh (Variables|Default|GetSkeletalMesh))
  (bind _targetref (Variables|Default|GetTargetRef))
  (bind _returnvalue (Transformation|GetWorldLocation _skeletalmesh))
  (bind _returnvalue_2 (Transformation|GetActorLocation _targetref))
  (bind _returnvalue_3 (Math|Rotator|FindLookatRotation _returnvalue _returnvalue_2))
  (Utilities|IsValid (Variables|Default|GetTargetRef)
    (:Is%20Valid
      (Transformation|SetWorldRotation (Variables|Default|GetSkeletalMesh) (Math|Rotator|MakeRotator (.roll _defaultrotation) (.pitch _defaultrotation) (.yaw (Math|Interpolation|RInterpTo (Transformation|GetWorldRotation (Variables|Default|GetSkeletalMesh)) (Math|Rotator|MakeRotator (.roll _returnvalue_3) (.pitch _returnvalue_3) (+ (.yaw _returnvalue_3) -9e+01)) 2.0 0.1))) false false))
    (:Is%20Not%20Valid
      (CallFunction|ReturntoRest))))

(fn CheckPuzzleActorState
  (return "Default"))