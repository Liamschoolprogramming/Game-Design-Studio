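; Flower obstacle that swivels its skeletal mesh to face the player inside its vision sphere and returns to its starting rotation afterward.
; Unless Disabled, sphere overlaps swap two looping timers: RotateToTarget tracks the player's yaw, while GoBack eases back to the BeginPlay rotation.
; Both loops add the inverse of the remaining yaw difference to RInterpTo's delta time, so the turn keeps pace as it nears its target.
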(event OnComponentBeginOverlap(VisionSphere)
  (params (OverlappedComponent :type Primitive%20Component%20Object%20Reference) (OtherActor :type Actor%20Object%20Reference) (OtherComp :type Primitive%20Component%20Object%20Reference) (OtherBodyIndex :type Integer) (bFromSweep :type Boolean) (SweepResult :type Hit%20Result%20Structure%20%28by%20ref%29))
  ;[0.15 0.15 0.15 0.5] When player setps into vision range, rotate to face player
  (if (and (Class|GameplayStatics|ObjectIsA OtherActor "/Script/GameDesignStudio.PlayerCharacter") (not (Class|GameplayStatics|ObjectIsA OtherComp "/Script/Engine.SphereComponent")))
    (Variables|Default|SetTargetRef OtherActor)
    (if (not (Variables|Default|GetbDisabled))
      (Utilities|Time|ClearandInvalidateTimerbyHandle (Variables|Default|GetReturnRotateTimer))
      (bind _returnvalue (Utilities|Time|SetTimerbyFunctionName 0 "RotateToTarget" 0.01 true true))
      (Variables|Default|SetAttackRotateTimer _returnvalue))))

(event OnComponentEndOverlap(VisionSphere)
  (params (OverlappedComponent :type Primitive%20Component%20Object%20Reference) (OtherActor :type Actor%20Object%20Reference) (OtherComp :type Primitive%20Component%20Object%20Reference) (OtherBodyIndex :type Integer))
  ;[0.15 0.15 0.15 0.5] When player exits sight range,  return to rest
  (if (Class|GameplayStatics|ObjectIsA OtherActor "/Game/GameDesignStudio/Characters/BP_PlayerCharacter.BP_PlayerCharacter_C")
    (if (not (Variables|Default|GetbDisabled))
      (Utilities|Time|ClearandInvalidateTimerbyHandle (Variables|Default|GetFollowingTimer))
      (Utilities|Time|ClearandInvalidateTimerbyHandle (Variables|Default|GetFollowingTimer))
      (Variables|Default|SetTargetRef 0)
      (CallFunction|ReturntoRest))))

(event EventBeginPlay
  ;[0.15 0.15 0.15 0.5] Sets default rotation (which is also the rotation it will return to when player not visible)
  (Variables|Default|SetDefaultRotation (Transformation|GetActorRotation)))

(fn ConstructionScript
  (|CallParentFunction))

(fn Aim
  (params (Yaw :type Float%20%28double-precision%29))
  (bind _skeletalmesh (Variables|Default|GetSkeletalMesh))
  (bind _relativerotation (Variables|/Script/Engine.SceneComponent|GetRelativeRotation _skeletalmesh))
  ;[0.15 0.15 0.15 0.5] Rotates only left right movement input
  (Pawn|Input|AddControllerYawInput Yaw)
  (Transformation|SetRelativeRotation (Variables|Default|GetSkeletalMesh) (Math|Rotator|MakeRotator (.roll _relativerotation) (.pitch _relativerotation) (.yaw (Pawn|GetControlRotation :!class /Script/Engine.Pawn))) false false))

(fn ReturntoRest
  ;[0.15 0.15 0.15 0.5] Calls Loop To Return to Rest After Losing the Target
  (Utilities|Time|ClearandInvalidateTimerbyHandle (Variables|Default|GetAttackRotateTimer))
  (bind _returnvalue (Utilities|Time|SetTimerbyFunctionName 0 "GoBack" 0.01 true true))
  (Variables|Default|SetReturnRotateTimer _returnvalue))

(fn GoBack
  (bind _returnvalue (Utilities|Time|GetWorldDeltaSeconds))
  (bind _defaultrotation (Variables|Default|GetDefaultRotation))
  (bind _defaultrotation_2 (Variables|Default|GetDefaultRotation))
  (bind _skeletalmesh (Variables|Default|GetSkeletalMesh))
  (bind _skeletalmesh_2 (Variables|Default|GetSkeletalMesh))
  (bind _returnvalue_2 (Transformation|GetWorldRotation _skeletalmesh))
  (bind _returnvalue_3 (Transformation|GetWorldRotation _skeletalmesh_2))
  (bind _returnvalue_4 (Math|Rotator|Delta(Rotator) _returnvalue_3 _defaultrotation_2))
  (bind _returnvalue_5 (Math|Float|Absolute(Float) (.yaw _returnvalue_4)))
  (bind _returnvalue_6 (/ 1.0 _returnvalue_5))
  (bind _returnvalue_7 (+ _returnvalue _returnvalue_6))
  (bind _returnvalue_8 (Math|Interpolation|RInterpTo _returnvalue_2 _defaultrotation _returnvalue_7 0.5))
  ;[0.15 0.15 0.15 0.5] Loop that rotates head back to default rotation
  (Transformation|SetWorldRotation (Variables|Default|GetSkeletalMesh) (Math|Rotator|MakeRotator (.roll (Transformation|GetWorldRotation (Variables|Default|GetSkeletalMesh))) (.pitch _returnvalue_8) (.yaw _returnvalue_8)) false false)
  (if (== (Math|Float|Round (.yaw (Transformation|GetWorldRotation (Variables|Default|GetSkeletalMesh)))) (Math|Float|Round (.yaw (Variables|Default|GetDefaultRotation))))
    (Utilities|Time|ClearandInvalidateTimerbyHandle (Variables|Default|GetReturnRotateTimer))))

(fn RotatetoTarget
  (bind _skeletalmesh (Variables|Default|GetSkeletalMesh))
  (bind _skeletalmesh_2 (Variables|Default|GetSkeletalMesh))
  (bind _skeletalmesh_3 (Variables|Default|GetSkeletalMesh))
  (bind _targetref (Variables|Default|GetTargetRef))
  (bind _returnvalue (Transformation|GetWorldLocation _skeletalmesh_3))
  (bind _returnvalue_2 (Transformation|GetWorldRotation _skeletalmesh_2))
  (bind _returnvalue_3 (Transformation|GetActorLocation _targetref))
  (bind _relativerotation (Variables|/Script/Engine.SceneComponent|GetRelativeRotation _skeletalmesh))
  (bind _returnvalue_4 (Math|Rotator|FindLookatRotation _returnvalue _returnvalue_3))
  (bind _returnvalue_5 (+ (.yaw _returnvalue_4) -9e+01))
  (bind _returnvalue_6 (Math|Rotator|MakeRotator (.roll _returnvalue_4) (.pitch _returnvalue_4) _returnvalue_5))
  (Utilities|IsValid (Variables|Default|GetTargetRef)
    (:Is%20Valid
      (Transformation|SetWorldRotation (Variables|Default|GetSkeletalMesh) (Math|Rotator|MakeRotator (.roll _relativerotation) (.pitch _relativerotation) (.yaw (Math|Interpolation|RInterpTo _returnvalue_2 _returnvalue_6 (+ (Utilities|Time|GetWorldDeltaSeconds) (/ 1.0 (Math|Float|Absolute(Float) (.yaw (Math|Rotator|Delta(Rotator) _returnvalue_2 _returnvalue_6))))) 0.5))) false false))
    (:Is%20Not%20Valid
      (CallFunction|ReturntoRest))))

(fn CheckPuzzleActorState
  (return "Default"))