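; Roaming hazard that patrols MovePoints and carries a gloom sphere that damages the player.
; Tick moves it toward the current point, pausing on arrival, while a sphere trace sends it back a point when a boulder or vine blockade is ahead.
; Overlapping the player hitbox starts looping damage; the Inverted puzzle state stops damage and the Niagara effect.
; Budding Turret shots stun its movement temporarily.
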(event OnComponentBeginOverlap(Gloomspace)
  (params (OverlappedComponent :type Primitive%20Component%20Object%20Reference) (OtherActor :type Actor%20Object%20Reference) (OtherComp :type Primitive%20Component%20Object%20Reference) (OtherBodyIndex :type Integer) (bFromSweep :type Boolean) (SweepResult :type Hit%20Result%20Structure%20%28by%20ref%29))
  ;[0.15 0.15 0.15 0.5] damage zone stuff
  (if (and (Components|ComponentHasTag OtherComp "PlayerHitBox") (not (Utilities|Enum|Equal(Enum) (Variables|Default|GetPuzzleElementState) "Inverted")))
    (bind _output_get (Variables|Default|SetDamagedActor OtherActor))
    (Game|Damage|ApplyDamage _output_get 0.5 0 0)
    (bind _returnvalue (Utilities|Time|SetTimerbyEvent (delegate Custom|DamagePlayer) 1.0 true true))
    (Variables|Default|SetGloomTimer _returnvalue)))

(event OnComponentEndOverlap(Gloomspace)
  (params (OverlappedComponent :type Primitive%20Component%20Object%20Reference) (OtherActor :type Actor%20Object%20Reference) (OtherComp :type Primitive%20Component%20Object%20Reference) (OtherBodyIndex :type Integer))
  (bind _gloomtimer (Variables|Default|GetGloomTimer))
  ;[0.15 0.15 0.15 0.5] damage zone stuff
  (if (and (Components|ComponentHasTag OtherComp "PlayerHitBox") (Utilities|Time|IsValidTimerHandle _gloomtimer))
    (Development|PrintString "LEAVING")
    (Utilities|Time|ClearandInvalidateTimerbyHandle _gloomtimer)))

(event Custom|DamagePlayer
  ;[0.15 0.15 0.15 0.5] damage zone stuff
  (Game|Damage|ApplyDamage (Variables|Default|GetDamagedActor) 0.5 0 0))

(event Custom|DecrementMove
  ;[0.15 0.15 0.15 0.5] decrement move point
  (Variables|Default|SetDecrementingAlready? false)
  (bind _result (Math|Integer|DecrementInt (Variables|Default|GetMoveTick))
    (:%20%20
      (if (< _result 0)
        (Variables|Default|SetMoveTick (- (Utilities|Array|Length (Variables|Default|GetMovePoints)) 1)))
      (Transformation|SetActorRotation (Math|Rotator|MakeRotator 0.0 0.0 (.yaw (Math|Rotator|FindLookatRotation (Transformation|GetActorLocation) (Utilities|Array|Get(acopy) (Variables|Default|GetMovePoints) (Variables|Default|GetMoveTick))))))
      (Variables|Default|SetCanMove? true))))

(event Custom|IncrementMove
  ;[0.15 0.15 0.15 0.5] tick movement up
  (bind _result (Math|Integer|IncrementInt (Variables|Default|GetMoveTick))
    (:%20%20
      (if (> _result (- (Utilities|Array|Length (Variables|Default|GetMovePoints)) 1))
        (Variables|Default|SetMoveTick 0))
      (Transformation|SetActorRotation (Math|Rotator|MakeRotator 0.0 0.0 (.yaw (Math|Rotator|FindLookatRotation (Transformation|GetActorLocation) (Utilities|Array|Get(acopy) (Variables|Default|GetMovePoints) (Variables|Default|GetMoveTick))))))
      (Variables|Default|SetCanMove? true)
      (Variables|Default|SetDecrementingAlready? false))))

(event Custom|FinishStun
  ;[0.15 0.15 0.15 0.5] Budding Turret Projectile Interaction
  (Variables|Default|SetCanMove? true))

(event EventTick
  (params (DeltaSeconds :type Float%20%28single-precision%29))
  (bind _returnvalue (Transformation|GetActorLocation))
  (bind _returnvalue_2 (Transformation|GetActorLocation))
  ;[0.15 0.15 0.15 0.5] walking
  (if (Variables|Default|GetCanMove?)
    (Transformation|SetActorLocation (+ _returnvalue (* (Math|Vector|Normalize (- (Utilities|Array|Get(acopy) (Variables|Default|GetMovePoints) (Variables|Default|GetMoveTick)) _returnvalue)) (* DeltaSeconds (Variables|Default|GetSpeed)))) false true)
    (if (<= (Math|Vector|Distance(Vector) (Transformation|GetActorLocation) (Utilities|Array|Get(acopy) (Variables|Default|GetMovePoints) (Variables|Default|GetMoveTick))) 5e+01)
      (Variables|Default|SetCanMove? false)
      (Utilities|Time|SetTimerbyEvent (delegate Custom|IncrementMove) 2.0 false true)
      (elif (not (Variables|Default|GetDecrementingAlready?))
        (bind _outhit (Collision|SphereTraceByChannel (+ _returnvalue_2 "0.000000,0.000000,50.000000") (+ _returnvalue_2 (* (Math|Vector|Normalize (- (Utilities|Array|Get(acopy) (Variables|Default|GetMovePoints) (Variables|Default|GetMoveTick)) _returnvalue_2)) 2e+02) "0.000000,0.000000,50.000000") 5e+01 "TraceTypeQuery4" false 0 "ForOneFrame"))
        (Utilities|Casting|CastToBP_Boulder (.HitActor (Collision|BreakHitResult _outhit))
          (:then
            _)
          (:CastFailed
            (Utilities|Casting|CastToBP_VineBlockade (.HitActor (Collision|BreakHitResult _outhit)))))
        (Variables|Default|SetDecrementingAlready? true)
        (Utilities|Time|SetTimerbyEvent (delegate Custom|DecrementMove) 0.5 false true)))))

(event EventShotbyBuddingTurret
  ;[0.15 0.15 0.15 0.5] Budding Turret Projectile Interaction
  (Variables|Default|SetCanMove? false)
  (Utilities|Time|SetTimerbyEvent (delegate Custom|FinishStun) 5.0 false true))

(event EventChangePuzzleActorState
  (params (EPuzzleState :type EPuzzleElementState%20Enum :default "Default"))
  (bind _gloomtimer (Variables|Default|GetGloomTimer))
  ;[0.15 0.15 0.15 0.5] inverter stuff
  (bind _output_get (Variables|Default|SetPuzzleElementState EPuzzleState))
  (switch Utilities|FlowControl|Switch|SwitchonEPuzzleElementState _output_get
    (:Default
      (if (not (Components|Activation|IsActive (Variables|Default|GetNS_GloomZone)))
        (Components|Activation|Activate (Variables|Default|GetNS_GloomZone) true)))
    (:Inverted
      (if (Utilities|Time|IsValidTimerHandle _gloomtimer)
        (Utilities|Time|ClearandInvalidateTimerbyHandle _gloomtimer))
      (Components|Activation|Deactivate (Variables|Default|GetNS_GloomZone)))))

(event EventBeginPlay
  (bind _gloomradius (Variables|Default|GetGloomRadius))
  (CallFunction|IncrementMove)
  (Components|Sphere|SetSphereRadius (Variables|Default|GetGloomspace) _gloomradius true)
  (Niagara|SetNiagaraVariable(Float) (Variables|Default|GetNS_GloomZone) "SphereRadius" _gloomradius))

(fn ConstructionScript
  (bind _ns_gloomzone (Variables|Default|GetNS_GloomZone))
  (Niagara|SetNiagaraVariable(Float) _ns_gloomzone "Loop Duration" (Variables|Default|GetDamageFrequency))
  (Niagara|SetNiagaraVariable(Vector3) _ns_gloomzone "SpriteFacing" "0, 0, 0"))

(fn CheckPuzzleActorState
  (return "Default"))