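; BP_DamageWall is a puzzle obstacle that damages overlapping actors, knocks back the player character and can be lowered by a pressure plate.
; BeginPlay stores the blocking height, and overlap applies damage before calling DoKnockback on the player.
; The PressurePlate event plays or reverses the Descend timeline, which offsets the wall's Z down by up to OpenDepth.
; CheckPuzzleActorState only returns a default value.
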(event EventBeginPlay
  ;[0.15 0.15 0.15 0.5] Set default z-position (blocking player)
  (Variables|Default|SetDefaultZPosition (.z (Transformation|GetActorLocation))))

(event Collision|EventActorBeginOverlap
  (params (OtherActor :type Actor%20Object%20Reference))
  (Game|Damage|ApplyDamage OtherActor (Variables|Default|GetDamage) 0 self)
  (bind _asplayer_character (Utilities|Casting|CastToPlayerCharacter OtherActor))
  (Class|PlayerCharacter|DoKnockback _asplayer_character (Variables|Default|GetKnockbackPower) self))

(event EventPressurePlate
  (params (Down? :type Boolean))
  (bind _returnvalue (Transformation|GetActorLocation))
  ;[0.15 0.15 0.15 0.5] Open door (play/true) or close door (reverse/false)
  (if Down?
    (bind _down (Timeline|Descend Play)
      (:Update
        (Transformation|SetActorLocation (Math|Vector|MakeVector (.x _returnvalue) (.y _returnvalue) (- (Variables|Default|GetDefaultZPosition) (* _down (Variables|Default|GetOpenDepth)))) false false)))
    (else
      (Timeline|Descend Reverse))))

(fn ConstructionScript)

(fn CheckPuzzleActorState
  (return "Default"))