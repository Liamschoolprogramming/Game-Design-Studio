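; BP_GriefObject is a placed actor that shows a grief particle effect which can be switched on and off.
; On BeginPlay it fetches its owning manager by class from the GameManagerSubsystem and registers itself as a grief actor.
; EnableGrief restarts the Niagara particle component, and DisableGrief deactivates it and prints a debug message.
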(event EventBeginPlay
  ;[0.15 0.15 0.15 0.5] afaik this is the only way it will work :(
  (bind _returnvalue (Class|GameManagerSubsystem|GetManagerbyClass (Subsystems|GetGameManagerSubsystem) (Variables|Default|GetOwningManager)))
  (Class|PuzzleGriefManager|RegisterGriefActor _returnvalue self))

(fn ConstructionScript)

(fn DisableGrief
  (Components|Activation|Deactivate (Variables|Default|GetNS_GriefParticles))
  (Development|PrintString "Grief should be disabled for this instance."))

(fn EnableGrief
  (Components|Activation|Activate (Variables|Default|GetNS_GriefParticles) true))