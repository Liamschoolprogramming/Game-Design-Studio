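; BP_PlayerTriggerNPCAction is a trigger volume that applies an action to a named NPC when the player overlaps it.
; The overlap, gated by a PlayerHitBox tag on the overlapped component, searches all BP_NPC_Base actors for a matching name.
; ExecuteNPCAction then optionally teleports that NPC and swaps its dialogue asset.
; A completion flag prevents repeats after success, while a missing NPC only prints an error.
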(event OnComponentBeginOverlap(Box)
  (params (OverlappedComponent :type Primitive%20Component%20Object%20Reference) (OtherActor :type Actor%20Object%20Reference) (OtherComp :type Primitive%20Component%20Object%20Reference) (OtherBodyIndex :type Integer) (bFromSweep :type Boolean) (SweepResult :type Hit%20Result%20Structure%20%28by%20ref%29))
  (if (not (Variables|Default|GetbActionCompleted))
    (Utilities|Casting|CastToBP_PlayerCharacter OtherActor)
    (if (Components|ComponentHasTag OverlappedComponent "PlayerHitBox")
      (bind _outactors (Actor|GetAllActorsOfClass "/Game/GameDesignStudio/Characters/BP_NPC_Base.BP_NPC_Base_C"))
      (for _array_element _outactors
        (if (== (Variables|/Game/GameDesignStudio/Characters/BP_NPC_Base.BP_NPC_Base_C|GetName _array_element) (Variables|Default|GetNPC%20Name))
          (Variables|Default|SetNPCForAction _array_element)))
      (CallFunction|ExecuteNPCAction))))

(fn ConstructionScript)

(fn ExecuteNPCAction
  (Utilities|IsValid (Variables|Default|GetNPCForAction)
    (:Is%20Valid
      (if (Variables|Default|GetbShouldTeleport)
        (Transformation|SetActorLocation (Variables|Default|GetNPCForAction) (Variables|Default|GetTeleportLocation) false false))
      (if (Variables|Default|GetbShouldChangeDialogAsset)
        (Default|SetDialogueAsset (Variables|Default|GetNPCForAction) (Variables|Default|GetDialogAsset)))
      (Variables|Default|SetbActionCompleted true))
    (:Is%20Not%20Valid
      (Development|PrintString "No matching NPC found!"))))