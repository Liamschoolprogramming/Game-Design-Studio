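; BP_TestPressure_Plate is a test pressure plate that sinks when something overlaps its Sphere and tells a linked Corresponder to activate a door.
; Overlap begin calls ActivateDoor and plays the Press timeline, while overlap end calls DeactivateDoor and reverses it.
; The timeline lowers the whole actor from its starting Z by up to SinkDistance, setting PressedDown when it is within a small tolerance of the bottom.
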(event OnComponentBeginOverlap(Sphere)
  (params (OverlappedComponent :type Primitive%20Component%20Object%20Reference) (OtherActor :type Actor%20Object%20Reference) (OtherComp :type Primitive%20Component%20Object%20Reference) (OtherBodyIndex :type Integer) (bFromSweep :type Boolean) (SweepResult :type Hit%20Result%20Structure%20%28by%20ref%29))
  (bind _returnvalue (Transformation|GetActorLocation))
  (Default|ActivateDoor (Variables|Default|GetCorresponder))
  (bind _pressdistance (Timeline|Press Play)
    (:Update
      (Transformation|SetActorLocation (Math|Vector|MakeVector (.x _returnvalue) (.y _returnvalue) (- (Variables|Default|GetDefaultZPosition) (* _pressdistance (Variables|Default|GetSinkDistance)))) false false)
      (if (<= (.z (Transformation|GetActorLocation)) (+ (- (Variables|Default|GetDefaultZPosition) (Variables|Default|GetSinkDistance)) 0.1))
        (Variables|Default|SetPressedDown true)
        (else
          (Variables|Default|SetPressedDown false))))))

(event OnComponentEndOverlap(Sphere)
  (params (OverlappedComponent :type Primitive%20Component%20Object%20Reference) (OtherActor :type Actor%20Object%20Reference) (OtherComp :type Primitive%20Component%20Object%20Reference) (OtherBodyIndex :type Integer))
  (bind _returnvalue (Transformation|GetActorLocation))
  (Default|DeactivateDoor (Variables|Default|GetCorresponder))
  (bind _pressdistance (Timeline|Press Reverse)
    (:Update
      (Transformation|SetActorLocation (Math|Vector|MakeVector (.x _returnvalue) (.y _returnvalue) (- (Variables|Default|GetDefaultZPosition) (* _pressdistance (Variables|Default|GetSinkDistance)))) false false)
      (if (<= (.z (Transformation|GetActorLocation)) (+ (- (Variables|Default|GetDefaultZPosition) (Variables|Default|GetSinkDistance)) 0.1))
        (Variables|Default|SetPressedDown true)
        (else
          (Variables|Default|SetPressedDown false))))))

(event EventBeginPlay
  (Variables|Default|SetDefaultZPosition (.z (Transformation|GetActorLocation))))

(fn ConstructionScript)