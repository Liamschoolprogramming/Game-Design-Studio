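; BP_Test_Door is a test door that slides vertically open and closed through ActivateDoor and DeactivateDoor events.
; BeginPlay caches the mesh's world Z, and the DoorOpen timeline plays or reverses to offset that height by up to OpenHeight.
; Each update sets DoorOpened by comparing the actor's Z, rather than the moving mesh's, against a threshold just below the open height.
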(event Custom|ActivateDoor
  (bind _doormesh (Variables|Default|GetDoorMesh))
  (bind _returnvalue (Transformation|GetWorldLocation _doormesh))
  (bind _dooropen (Timeline|DoorOpen Play)
    (:Update
      (Transformation|SetWorldLocation (Variables|Default|GetDoorMesh) (Math|Vector|MakeVector (.x _returnvalue) (.y _returnvalue) (+ (Variables|Default|GetDefaultZPosition) (* _dooropen (Variables|Default|GetOpenHeight)))) false false)
      (if (<= (.z (Transformation|GetActorLocation)) (- (+ (Variables|Default|GetDefaultZPosition) (Variables|Default|GetOpenHeight)) 0.1))
        (Variables|Default|SetDoorOpened true)
        (else
          (Variables|Default|SetDoorOpened false))))))

(event Custom|DeactivateDoor
  (bind _doormesh (Variables|Default|GetDoorMesh))
  (bind _returnvalue (Transformation|GetWorldLocation _doormesh))
  (bind _dooropen (Timeline|DoorOpen Reverse)
    (:Update
      (Transformation|SetWorldLocation (Variables|Default|GetDoorMesh) (Math|Vector|MakeVector (.x _returnvalue) (.y _returnvalue) (+ (Variables|Default|GetDefaultZPosition) (* _dooropen (Variables|Default|GetOpenHeight)))) false false)
      (if (<= (.z (Transformation|GetActorLocation)) (- (+ (Variables|Default|GetDefaultZPosition) (Variables|Default|GetOpenHeight)) 0.1))
        (Variables|Default|SetDoorOpened true)
        (else
          (Variables|Default|SetDoorOpened false))))))

(event EventBeginPlay
  (Variables|Default|SetDefaultZPosition (.z (Transformation|GetWorldLocation (Variables|Default|GetDoorMesh)))))

(fn ConstructionScript)