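; BP_TestColumn is a test column that topples once when the player character first overlaps its trigger box.
; The overlap passes a DoOnce into PillarFall, which plays the FallDown timeline to rotate the cylinder's pitch up to 90 degrees per unit of curve value from its BeginPlay pitch.
; Each update also prints the pitch for debugging, and an unused SetActorRotation node remains disconnected.
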(event OnComponentBeginOverlap(Box)
  (params (OverlappedComponent :type Primitive%20Component%20Object%20Reference) (OtherActor :type Actor%20Object%20Reference) (OtherComp :type Primitive%20Component%20Object%20Reference) (OtherBodyIndex :type Integer) (bFromSweep :type Boolean) (SweepResult :type Hit%20Result%20Structure%20%28by%20ref%29))
  (if (Class|GameplayStatics|ObjectIsA OtherActor "/Game/GameDesignStudio/Characters/BP_PlayerCharacter.BP_PlayerCharacter_C")
    (Utilities|FlowControl|DoOnce false
      (:Completed
        (CallFunction|PillarFall)))))

(event Custom|PillarFall
  (bind _cylinder (Variables|Default|GetCylinder))
  (bind _returnvalue (Transformation|GetWorldRotation _cylinder))
  (bind _rotation (Timeline|FallDown PlayFromStart)
    (:Update
      (Transformation|SetWorldRotation (Variables|Default|GetCylinder) (Math|Rotator|MakeRotator (.roll _returnvalue) (- (Variables|Default|GetDefaultPitch) (* _rotation -9e+01)) (.yaw _returnvalue)) false false)
      (Development|PrintString (Utilities|String|ToString(Float) (- (Variables|Default|GetDefaultPitch) (* _rotation -9e+01)))))))

(event EventBeginPlay
  (Variables|Default|SetDefaultPitch (.pitch (Transformation|GetWorldRotation (Variables|Default|GetCylinder)))))

(fn ConstructionScript)