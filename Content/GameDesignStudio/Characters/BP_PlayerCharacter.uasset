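; Player character Blueprint for Juniper, handling health, death, respawn, double jump and dash.
; BeginPlay places the player at the return point matching the game instance's last level.
; Death swaps the body for a staff mesh and shows the respawn screen; respawn uses the active save station or PlayerStart.
; Dash uses timeline-driven launches with movement locked and a cooldown; commented stamina gates are hard-wired true, and debug keys cycle stations or self-damage.
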(event Custom|Dash
  ;[0.15 0.15 0.15 0.5] Dash: If the player's stamina stat >= 10, dash forward (disabling other movement during the 0.4 sec duration); Has a cooldown of 0.5 sec
  (bind _bp_player_controller (Class|BPIPlayerControllerPossession|GetBPPlayerController(Message) (Pawn|GetController)))
  (Variables|/Script/GameDesignStudio.PlayerControllerBase|SetbCanMove _bp_player_controller false)
  (bind _distance (Timeline|Timeline PlayFromStart)
    (:Update
      (Character|LaunchCharacter (* (* (* _distance 3e+02) (Math|Vector|GetForwardVector (Transformation|GetActorRotation))) (* (Utilities|Time|GetWorldDeltaSeconds) 6e+01)) false false))
    (:Finished
      (Character|LaunchCharacter (Math|Vector|GetForwardVector (Transformation|GetActorRotation)) true true)
      (bind _bp_player_controller_2 (Class|BPIPlayerControllerPossession|GetBPPlayerController(Message) (Pawn|GetController)))
      (Variables|/Script/GameDesignStudio.PlayerControllerBase|SetbCanMove _bp_player_controller_2 true)
      (bind _returnvalue (Utilities|Time|SetTimerbyFunctionName 0 "ResetCanDash" 0.5))
      (Variables|Default|SetDashCooldown _returnvalue))))

(event Custom|PlayRunAnim
  (bind _asabp_juniper (Utilities|Casting|CastToABP_Juniper (Components|SkeletalMesh|GetAnimInstance (Variables|Default|GetSkeletalMesh))))
  (Default|SetIsRunning _asabp_juniper true))

(event Custom|StopRunAnim
  (bind _asabp_juniper (Utilities|Casting|CastToABP_Juniper (Components|SkeletalMesh|GetAnimInstance (Variables|Default|GetSkeletalMesh))))
  (Default|SetIsRunning _asabp_juniper false))

(event Input|EnhancedActionEvents|EnhancedInputActionIA_Jump
  (params (ActionValue :type Boolean) (ElapsedSeconds :type Float%20%28double-precision%29) (TriggeredSeconds :type Float%20%28double-precision%29) (InputAction :type Input%20Action%20Object%20Reference :default "/Game/GameDesignStudio/Input/Actions/IA_Jump.IA_Jump"))
  ;[0.15 0.15 0.15 0.5] Jump: If the player's stamina stat is >= 5, they can double jump; Otherwise, the jump count is capped at 1
  (:Started
    (if true
      (Variables|Default|SetJumpMaxCount 2)
      (Character|Jump)
      (else
        (Variables|Default|SetJumpMaxCount 1)
        (Character|Jump)))
    (bind _asabp_juniper (Utilities|Casting|CastToABP_Juniper (Components|SkeletalMesh|GetAnimInstance (Variables|Default|GetSkeletalMesh))))
    (Default|Jump _asabp_juniper)))

(event Input|EnhancedActionEvents|EnhancedInputActionIA_Dash
  (params (ActionValue :type Boolean) (ElapsedSeconds :type Float%20%28double-precision%29) (TriggeredSeconds :type Float%20%28double-precision%29) (InputAction :type Input%20Action%20Object%20Reference :default "/Game/GameDesignStudio/Input/Actions/IA_Dash.IA_Dash"))
  ;[0.15 0.15 0.15 0.5] Dash: If the player's stamina stat >= 10, dash forward (disabling other movement during the 0.4 sec duration); Has a cooldown of 0.5 sec
  (:Started
    (if true
      (if (Variables|Default|GetCanDash?)
        (bind _asplayer_controller_base (Utilities|Casting|CastToPlayerControllerBase (Game|GetPlayerController 0)))
        (if (not (Variables|/Script/GameDesignStudio.PlayerControllerBase|GetIsPossessing _asplayer_controller_base))
          (Variables|Default|SetCanDash? false)
          (CallFunction|Dash)
          (bind _returnvalue (UserInterface|CreateWidget "/Game/GameDesignStudio/UI/DashBar/WBP_DashBar.WBP_DashBar_C" (Game|GetPlayerController 0)))
          (UserInterface|Viewport|AddtoViewport _returnvalue 0)
          (Utilities|FlowControl|Delay 0.5)
          (Widget|RemovefromParent _returnvalue))))))

(event EventBeginPlay
  ;[0.15 0.15 0.15 0.5] Setup
  (Variables|Default|SetHealth (Variables|Default|GetMaxHealth))
  (CallFunction|SetDefaultLocation))

(event Game|Damage|EventAnyDamage
  (params (Damage :type Float%20%28single-precision%29) (DamageType :type Damage%20Type%20Object%20Reference) (InstigatedBy :type Controller%20Object%20Reference) (DamageCauser :type Actor%20Object%20Reference))
  ;[0.04766 0.3177 0.04766 0.5] Health System
  ;;[0.15 0.15 0.15 0.5] When Damaged
  (Variables|Default|SetHealth (Math|Float|Clamp(Float) (- (Variables|Default|GetHealth) Damage) 0.0 (Variables|Default|GetMaxHealth)))
  (Class|BPIPlayerCharacter|OnHealthChanged(Message) (HUD|GetHUD (Game|GetPlayerController 0)))
  (if (== (Variables|Default|GetHealth) 0.0)
    (Class|PlayerCharacter|PlayerDeath)))

(event EventPlayerDeath
  ;[0.04766 0.3177 0.04766 0.5] Health System
  ;;[0.15 0.15 0.15 0.5] Player Death
  (if (not (Variables|Default|GetIsPlayerDead))
    (CallFunction|PlayerDead)))

(event EventPlayerRespawn
  ;[0.04766 0.3177 0.04766 0.5] Health System
  ;;[0.15 0.15 0.15 0.5] Player Respawn
  (Transformation|SetActorLocation (CallFunction|GetRespawnLocation) false true)
  (Components|StaticMesh|SetStaticMesh (Variables|Default|GetStaticMesh_TPP) 0)
  (Components|SkeletalMesh|SetSkeletalMeshAsset (Variables|Default|GetSkeletalMesh) "/Game/GameDesignStudio/Characters/Juniper/SK_Juniper.SK_Juniper")
  (Variables|Default|SetIsPlayerDead false)
  (Variables|Default|SetHealth (Variables|Default|GetMaxHealth))
  (Class|BPIPlayerCharacter|OnHealthChanged(Message) (HUD|GetHUD (Game|GetPlayerController 0))))

(event Input|KeyboardEvents|Hyphen
  (params (Key :type Key%20Structure :default "None"))
  ;[1 0.1913 0 0.5] Debug Save Station Cycling
  ;;[0.15 0.15 0.15 0.5] Previous Save Station
  (:Pressed
    (Class|SaveStationManager|PreviousSaveStation (Class|GameManagerSubsystem|GetSaveStationManager (Subsystems|GetGameManagerSubsystem)))
    (Class|PlayerCharacter|PlayerRespawn)))

(event Input|KeyboardEvents|R
  (params (Key :type Key%20Structure :default "None"))
  ;[0.04766 0.3177 0.04766 0.5] Health System
  ;;[1 0.1913 0 0.5] Debug Self Damage
  (:Pressed
    (Game|Damage|ApplyDamage self 1.0 0 0)))

(event Input|KeyboardEvents|Equals
  (params (Key :type Key%20Structure :default "None"))
  ;[1 0.1913 0 0.5] Debug Save Station Cycling
  ;;[0.15 0.15 0.15 0.5] Next Save Station
  (:Pressed
    (Class|SaveStationManager|NextSaveStation (Class|GameManagerSubsystem|GetSaveStationManager (Subsystems|GetGameManagerSubsystem)))
    (Class|PlayerCharacter|PlayerRespawn)))

(fn ConstructionScript)

(fn ResetCanDash
  (Variables|Default|SetCanDash? true))

(fn GetRespawnLocation
  (bind _returnvalue (Subsystems|GetGameManagerSubsystem))
  (bind _returnvalue_2 (Class|GameManagerSubsystem|GetSaveStationManager _returnvalue))
  (bind _activesavestation (Variables|/Script/GameDesignStudio.SaveStationManager|GetActiveSaveStation _returnvalue_2))
  (Utilities|IsValid _activesavestation
    (:Is%20Valid
      ;[0.15 0.15 0.15 0.5] Save Station Exists, Use Its Location
      (return (+ (Transformation|GetActorLocation _activesavestation) (Variables|/Script/GameDesignStudio.SaveStation|GetSpawnLocation _activesavestation))))
    (:Is%20Not%20Valid
      ;[0.15 0.15 0.15 0.5] No Save Station, Use Player Start
      (bind _returnvalue_3 (Actor|GetActorOfClass "/Script/Engine.PlayerStart"))
      (return (Transformation|GetActorLocation _returnvalue_3)))))

(fn SetDefaultLocation
  (bind _asbp_elsgame_instance (Utilities|Casting|CastToBP_ELSGameInstance (Game|GetGameInstance)))
  (bind _outactors (Actor|GetAllActorsOfClass "/Game/GameDesignStudio/Warps/BP_ReturnPoint.BP_ReturnPoint_C"))
  (for _array_element _outactors
    (if (== (Variables|/Game/GameDesignStudio/Warps/BP_ReturnPoint.BP_ReturnPoint_C|GetLevelComingFrom _array_element) (Variables|/Game/GameDesignStudio/Core/BP_ELSGameInstance.BP_ELSGameInstance_C|GetLastLevel _asbp_elsgame_instance))
      (Transformation|SetActorLocationAndRotation (.Location (Math|Transform|BreakTransform (Transformation|GetActorTransform _array_element))) (.Rotation (Math|Transform|BreakTransform (Transformation|GetActorTransform _array_element))) false true)))
  (bind _returnvalue (Game|GetCurrentLevelName true))
  (Variables|/Game/GameDesignStudio/Core/BP_ELSGameInstance.BP_ELSGameInstance_C|SetLastLevel _asbp_elsgame_instance _returnvalue))

(fn PlayerDead
  (Variables|Default|SetIsPlayerDead true)
  (Niagara|SpawnSystematLocation "/Game/GameDesignStudio/Effects/PlayerDeath/NS_PlayerDeath.NS_PlayerDeath" (+ (Transformation|GetActorLocation) (* (Math|Vector|VectorUp) 1.5e+02)))
  (Character|LaunchCharacter "0.000000,0.000000,250.000000" false true)
  (bind _asbp_hud (Utilities|Casting|CastToBP_HUD (HUD|GetHUD (Game|GetPlayerController 0))))
  (Default|DisplayRespawnScreen _asbp_hud)
  (Components|StaticMesh|SetStaticMesh (Variables|Default|GetStaticMesh_TPP) "/Game/GameDesignStudio/Characters/Juniper/S_JuniperStaff.S_JuniperStaff")
  (Components|SkeletalMesh|SetSkeletalMeshAsset (Variables|Default|GetSkeletalMesh) 0)
  (Input|SetInputModeUIOnly (Game|GetPlayerController 0) 0 "DoNotLock" true))