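; BP_NPC_Base is a base NPC that starts a dialogue when the player's hit box enters its sphere.
; The overlap calls OnOverlapWithPlayer, which passes the DialogueSpeakerComponent's asset to the Dialogue subsystem; the end-overlap handler is empty.
; Helper functions look up data table rows by name to unlock puzzle items through the Game Manager's inventory manager and possessable character types through the player controller.
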(event OnComponentBeginOverlap(Sphere)
  (params (OverlappedComponent :type Primitive%20Component%20Object%20Reference) (OtherActor :type Actor%20Object%20Reference) (OtherComp :type Primitive%20Component%20Object%20Reference) (OtherBodyIndex :type Integer) (bFromSweep :type Boolean) (SweepResult :type Hit%20Result%20Structure%20%28by%20ref%29))
  (if (Components|ComponentHasTag OtherComp "PlayerHitBox")
    (CallFunction|OnOverlapwithPlayer)))

(event OnComponentEndOverlap(Sphere)
  (params (OverlappedComponent :type Primitive%20Component%20Object%20Reference) (OtherActor :type Actor%20Object%20Reference) (OtherComp :type Primitive%20Component%20Object%20Reference) (OtherBodyIndex :type Integer))
  (if (Components|ComponentHasTag OtherComp "PlayerHitBox")
    (CallFunction|OnEndOverlapwithPlayer)))

(event EventBeginPlay)

(event Collision|EventActorBeginOverlap
  (params (OtherActor :type Actor%20Object%20Reference)))

(event EventTick
  (params (DeltaSeconds :type Float%20%28single-precision%29)))

(fn ConstructionScript)

(fn OnOverlapwithPlayer
  (bind _dialoguespeakercomponent (Variables|Default|GetDialogueSpeakerComponent))
  (bind _dialogueasset (Variables|/Script/DialogueAssetEditorRuntime.DialogueSpeakerComponent|GetDialogueAsset _dialoguespeakercomponent))
  (Utilities|IsValid _dialogueasset
    (:Is%20Valid
      (Class|DialogueSubsystem|StartDialogue (Subsystems|GetDialogueSubsystem) _dialogueasset self (Game|GetPlayerController 0)))))

(fn OnEndOverlapwithPlayer)

(fn UnlockPuzzleItem
  (params (PuzzleItemName :type Name))
  (bind _returnvalue (Utilities|GetDataTableRow "/Game/GameDesignStudio/UI/Inventory/PuzzleInventory/DT_PuzzleInventoryItems.DT_PuzzleInventoryItems" PuzzleItemName)
    (:then
      (Class|PuzzleInventoryManager|UnlockPuzzleItem (Class|GameManagerSubsystem|GetPuzzleInventoryManager (Subsystems|GetGameManagerSubsystem)) _returnvalue))))

(fn UnlockPossessable
  (params (PossessableName :type Name))
  (bind _returnvalue (Utilities|GetDataTableRow "/Game/GameDesignStudio/Possessables/DT_PlayerCharacterTypeIcon.DT_PlayerCharacterTypeIcon" PossessableName)
    (:then
      (bind _bp_player_controller (Class|BPIPlayerControllerPossession|GetBPPlayerController(Message) (Game|GetPlayerController 0)))
      (Class|PlayerControllerBase|UnlockPossession _bp_player_controller (.PlayerCharacterType (Utilities|Struct|BreakPlayerCharacterTypeIcon _returnvalue))))))