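; BP_PortalWarp is a portal that sends the player to another level when a component tagged PlayerHitBox overlaps its collision sphere.
; If confirmation is required, it passes the target level and name to the HUD's teleport prompt and shows it.
; Otherwise it plays a white fade widget and opens the level by object reference after a short fixed delay.
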(event OnComponentBeginOverlap(SphereCollision)
  (params (OverlappedComponent :type Primitive%20Component%20Object%20Reference) (OtherActor :type Actor%20Object%20Reference) (OtherComp :type Primitive%20Component%20Object%20Reference) (OtherBodyIndex :type Integer) (bFromSweep :type Boolean) (SweepResult :type Hit%20Result%20Structure%20%28by%20ref%29))
  (if (Components|ComponentHasTag OtherComp "PlayerHitBox")
    (if (Variables|Config|GetbRequiresConfirmation)
      ;[0.15 0.15 0.15 0.5] Confirmation Popup
      (bind _asbp_hud (Utilities|Casting|CastToBP_HUD (HUD|GetHUD (Game|GetPlayerController 0))))
      (Default|SetTarget (Variables|/Game/GameDesignStudio/UI/BP_HUD.BP_HUD_C|GetTeleportPrompt _asbp_hud) (Variables|Config|GetLevel) (Variables|Config|GetLevelName))
      (Default|ToggleTeleportPrompt _asbp_hud true)
      (else
        ;[0.15 0.15 0.15 0.5] Instant Teleport
        (bind _returnvalue (UserInterface|CreateWidget "/Game/GameDesignStudio/UI/WBP_WhiteFade.WBP_WhiteFade_C"))
        (UserInterface|Viewport|AddtoViewport _returnvalue 0)
        (Default|Fade _returnvalue)
        (Utilities|FlowControl|Delay 2.2)
        (Game|OpenLevel(byObjectReference) (Variables|Config|GetLevel))))))

(fn ConstructionScript)